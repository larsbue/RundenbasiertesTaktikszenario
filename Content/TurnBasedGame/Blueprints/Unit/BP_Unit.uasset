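; Grid-based unit actor for turn-based battles, taking its mesh, animation and stats from unit type data.
; A timeline moves it tile by tile along paths, blending location, rotation and a jump offset.
; Clamped HP, AP and MP setters broadcast stat changes and spawn floating numbers.
; Spell damage changes HP immediately, but numbers and hit or death animations wait for the spell animation's impact.
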(event `self.ReceiveBeginPlay`
  ;[1 1 1] set hp bar of unit to display healthpoints. also, always start in idle animation state.
  (`self.SetAnimationState` "NewEnumerator0")
  (bind _output_get (set `self.HpBar` (cast `/Game/TurnBasedGame/Blueprints/Unit/Widgets/W_HpBar` (`WidgetComponent.GetUserWidgetObject` (`self.Widget_HpBar`)) :!pure true)))
  (`/Game/TurnBasedGame/Blueprints/Unit/Widgets/W_HpBar.SetUnit` _output_get self))

(event `FollowPath`
  (params (Path :type "Array of IntPoint Structure"))
  ;[1 1 1] entry into unit walking flow. check if there are still elements in the given path. if so, continue to follow/the flow.
  (if (> (`KismetArrayLibrary.Array_Length` Path) 0)
    (set `self.CurrentPathToFollow` Path)
    (`self.OnUnitStartedWalking` self)
    (`self.ContinueFollowPath`)))

(event `ContinueFollowPath`
  (bind _timeline_unitmovement (`self.Timeline_UnitMovement`))
  (if (> (`KismetArrayLibrary.Array_Length` (`self.CurrentPathToFollow`)) 0)
    (`self.SetAnimationState` "NewEnumerator1")
    (set `self.PreviousTransform` (`self.GetTransform`))
    (`self.SetNextTransformLocation`)
    (`TimelineComponent.SetPlayRate` _timeline_unitmovement (/ (`TimelineComponent.GetTimelineLength` _timeline_unitmovement) (`self.MoveDurationPerTile`)))
    (bind (_direction _locationalpha _rotationalpha _jump) (`Timeline|Timeline_UnitMovement` :!via `PlayFromStart`)
      (:`Update`
        ;[1 1 1] set new location and rotation by using the update of the timeline to make it seem fluid.
        (`self.K2_SetActorLocationAndRotation` (+ (`self.GetNewLocation` _locationalpha) (`KismetMathLibrary.MakeVector` 0.0 0.0 (`KismetMathLibrary.SelectFloat` 0.0 _jump (`self.GetIsJumping`)))) (`self.GetNewRotation` _rotationalpha)))
      (:`Finished`
        ;[1 1 1] transmit the current path to follow and remove the current element of the path. repeat the process until finished.
        (`self.OnUnitReachNewTile` self (`|GetArrayItem` (`self.CurrentPathToFollow`)))
        (`KismetArrayLibrary.Array_Remove` (`self.CurrentPathToFollow`))
        (`self.ContinueFollowPath`)))
    (else
      ;[1 1 1] after walking is done, set animation state to idle and inform.
      (`self.SetAnimationState` "NewEnumerator0")
      (`self.OnUnitFinishedWalking` self))))

(event `Debug_Respawn`
  (`KismetSystemLibrary.Delay` 1.8)
  (`self.SetCurrentHp` (`.HP_Max_15_6E7147AD427713A02E1E65ABFF535596` (break `/Game/TurnBasedGame/Blueprints/Unit/Utilities/BPS_Unit_Stats` (`.Stats_8_59677AC742C58E50C0B0B8BFC3DDDE60` (break `/Game/TurnBasedGame/Blueprints/Unit/Utilities/BPS_Unit` (`self.UnitData`))))) true)
  (`self.SetAnimationState` "NewEnumerator5"))

(event `HideUnit`
  (`KismetSystemLibrary.Delay` 1.8)
  (if (not (`self.IsAlive`))
    (`self.K2_SetActorLocation` (-99999.0 -99999.0 -99999.0))))

(fn `BattleEnded`
  ;[1 1 1] actions performed when battle ends.
  (`self.ResetMp`)
  (`self.ResetAp`))

(fn `BattleStarted`
  ;[1 1 1] actions performed when battle is started.
  (set `self.TimeUnitCreated` (`GameplayStatics.GetTimeSeconds`))
  (`self.ResetMp`)
  (`self.ResetAp`))

(fn `CalculateCastingFaceRotation`
  (params (TargetIndex :type "IntPoint Structure (by ref)"))
  (returns (NewRotation :type "Rotator Structure"))
  (bind (_x _y) (`KismetMathLibrary.BreakVector3f` (`self.K2_GetActorLocation`)))
  (bind _transform_location (`KismetMathLibrary.BreakTransform` (break `/Game/TurnBasedGame/Blueprints/Grid/Utilities/BPS_DataTile` (`BlueprintMapLibrary.Map_Find` (`/Game/TurnBasedGame/Blueprints/Grid/BP_Grid.GridTiles` (`self.Grid`)) TargetIndex))))
  (bind (_x_2 _y_2) (`KismetMathLibrary.BreakVector3f` _transform_location))
  (return (`KismetMathLibrary.FindLookAtRotation` (`KismetMathLibrary.MakeVector` _x _y) (`KismetMathLibrary.MakeVector` _x_2 _y_2))))

(fn `CalculateHpDiffAndClampedMax`
  (params (Value :type Integer))
  (returns (Diff :type Integer) (ClampedMax :type Integer))
  (bind ((`HP_Current_14_DF3407B84715BA0A38CA43B0D88C8ED4` _hp_current) (`HP_Max_15_6E7147AD427713A02E1E65ABFF535596` _hp_max)) (break `/Game/TurnBasedGame/Blueprints/Unit/Utilities/BPS_Unit_Stats` (`.Stats_8_59677AC742C58E50C0B0B8BFC3DDDE60` (break `/Game/TurnBasedGame/Blueprints/Unit/Utilities/BPS_Unit` (`self.UnitData`)))))
  (return (- Value _hp_current) (`KismetMathLibrary.Clamp` Value 0 _hp_max)))

(fn `CalculateMpDiffAndClampedMax`
  (params (MpValue :type Integer))
  (returns (Diff :type Integer) (ClampedMax :type Integer))
  (bind ((`MP_Current_9_342C6130430EBE8DE80D35B13735B31E` _mp_current) (`MP_Max_18_2725B4A5464FC373D37D05BEE793A5A3` _mp_max)) (break `/Game/TurnBasedGame/Blueprints/Unit/Utilities/BPS_Unit_Stats` (`.Stats_8_59677AC742C58E50C0B0B8BFC3DDDE60` (break `/Game/TurnBasedGame/Blueprints/Unit/Utilities/BPS_Unit` (`self.UnitData`)))))
  (return (- MpValue _mp_current) (`KismetMathLibrary.Clamp` MpValue 0 _mp_max)))

(fn `CanCastSpell`
  (params (SpellData :type "/Game/TurnBasedGame/Blueprints/Battle/Spells/Utilities/BPS_SpellData Structure"))
  (returns (CanCast :type Boolean))
  (if (`KismetArrayLibrary.Array_Contains` (`.AvailableSpells_22_B8E89C4A46E2713CC7D8EEACAC0A8795` (break `/Game/TurnBasedGame/Blueprints/Unit/Utilities/BPS_Unit_Stats` (`.Stats_8_59677AC742C58E50C0B0B8BFC3DDDE60` (break `/Game/TurnBasedGame/Blueprints/Unit/Utilities/BPS_Unit` (`self.UnitData`))))) (`.Spell_4_BE14505B4C6395A0D6DC359116D559E2` (break `/Game/TurnBasedGame/Blueprints/Battle/Spells/Utilities/BPS_SpellData` (`local.SpellData`))))
    (if (>= (`.AP_Current_28_7EC55DEC44D3AF38452837AE51007BFF` (break `/Game/TurnBasedGame/Blueprints/Unit/Utilities/BPS_Unit_Stats` (`.Stats_8_59677AC742C58E50C0B0B8BFC3DDDE60` (break `/Game/TurnBasedGame/Blueprints/Unit/Utilities/BPS_Unit` (`self.UnitData`))))) (`.ActionPointsCost_2_B2DF245A493C6B748782FCAFA215B290` (break `/Game/TurnBasedGame/Blueprints/Battle/Spells/Utilities/BPS_SpellData_Requirements` (`.Requirements_18_4281FB654CB40E08FCC5939ED071E8A6` (break `/Game/TurnBasedGame/Blueprints/Battle/Spells/Utilities/BPS_SpellData` (`local.SpellData`))))))
      (return true)
      (else
        (return false)))
    (else
      (return false))))

(fn `GetAnimationState`
  (returns (State :type "/Game/TurnBasedGame/Ressources/Units/E_StateUnitAnimation Enum"))
  (bind _state (message `/Game/TurnBasedGame/Ressources/Units/BPI_UnitAnimation.GetUnitAnimationState` (`SkeletalMeshComponent.GetAnimInstance` (`self.SkeletalMesh`))))
  (return _state))

(fn `GetIsJumping`
  (returns (ReturnValue :type Boolean))
  (return (`KismetMathLibrary.NearlyEqual_FloatFloat` (.z (.location (`self.PreviousTransform`))) (.z (.location (`self.NextTransform`))) 5.0)))

(fn `GetNewLocation`
  (params (Alpha :type "Float (single-precision)"))
  (returns (ReturnValue :type "Vector Structure"))
  (bind _previoustransform_location (`KismetMathLibrary.BreakTransform` (`self.PreviousTransform`)))
  (bind _nexttransform_location (`KismetMathLibrary.BreakTransform` (`self.NextTransform`)))
  (return (`KismetMathLibrary.VLerp` _previoustransform_location _nexttransform_location Alpha)))

(fn `GetNewRotation`
  (params (Alpha :type "Float (single-precision)"))
  (returns (ReturnValue :type "Rotator Structure"))
  (bind (_previoustransform_location _previoustransform_rotation) (`KismetMathLibrary.BreakTransform` (`self.PreviousTransform`)))
  (bind (_nexttransform_location _nexttransform_rotation) (`KismetMathLibrary.BreakTransform` (`self.NextTransform`)))
  (return (`KismetMathLibrary.RLerp` _previoustransform_rotation _nexttransform_rotation Alpha true)))

(fn `HandleUnitCastSpell`
  (params (TargetIndex :type "IntPoint Structure") (SpellData :type "/Game/TurnBasedGame/Blueprints/Battle/Spells/Utilities/BPS_SpellData Structure"))
  (`self.K2_SetActorRotation` (`self.CalculateCastingFaceRotation` TargetIndex))
  (`self.SetAnimationState` "NewEnumerator2")
  ;[1 1 1] after casting a spell, modify ap of unit accordingly.
  (`self.ModifyCurrentAp` (- 0 (`.ActionPointsCost_2_B2DF245A493C6B748782FCAFA215B290` (break `/Game/TurnBasedGame/Blueprints/Battle/Spells/Utilities/BPS_SpellData_Requirements` (`.Requirements_18_4281FB654CB40E08FCC5939ED071E8A6` (break `/Game/TurnBasedGame/Blueprints/Battle/Spells/Utilities/BPS_SpellData` (`local.SpellData`)))))) true))

(fn `HandleUnitHitBySpell`
  (params (SpellDamageTrue :type "/Game/TurnBasedGame/Blueprints/Battle/Spells/Utilities/BPS_SpellData_Stats_True Structure") (SpellAnimation :type "/Game/TurnBasedGame/Blueprints/Battle/Spells/BP_SpellAnims Object Reference"))
  (bind _modifier_hp (break `/Game/TurnBasedGame/Blueprints/Battle/Spells/Utilities/BPS_SpellData_Stats_True` (`local.SpellDamageTrue`)))
  (`BlueprintMapLibrary.Map_Add` (`self.IncomingSpells`) SpellAnimation SpellDamageTrue)
  (add `/Game/TurnBasedGame/Blueprints/Battle/Spells/BP_SpellAnims.OnSpellAnimationHit` SpellAnimation (`|CreateDelegate` :!event `OnSpellAnimationHit`))
  (if (!= _modifier_hp 0)
    (`self.ModifyCurrentHp` _modifier_hp)
    (`self.SetTotalDamageAndHealingTakenForDebug` _modifier_hp)))

(fn `IsAlive`
  (returns (IsAlive :type Boolean))
  (return (> (`.HP_Current_14_DF3407B84715BA0A38CA43B0D88C8ED4` (break `/Game/TurnBasedGame/Blueprints/Unit/Utilities/BPS_Unit_Stats` (`.Stats_8_59677AC742C58E50C0B0B8BFC3DDDE60` (break `/Game/TurnBasedGame/Blueprints/Unit/Utilities/BPS_Unit` (`self.UnitData`))))) 0)))

(fn `ModifyCurrentAp`
  (params (Modifier :type Integer) (ShowNumber :type Boolean))
  (`self.SetCurrentAp` (+ Modifier (`.AP_Current_28_7EC55DEC44D3AF38452837AE51007BFF` (break `/Game/TurnBasedGame/Blueprints/Unit/Utilities/BPS_Unit_Stats` (`.Stats_8_59677AC742C58E50C0B0B8BFC3DDDE60` (break `/Game/TurnBasedGame/Blueprints/Unit/Utilities/BPS_Unit` (`self.UnitData`)))))) ShowNumber))

(fn `ModifyCurrentHp`
  (params (Modifier :type Integer) (ShowNumber :type Boolean))
  (`self.SetCurrentHp` (+ Modifier (`.HP_Current_14_DF3407B84715BA0A38CA43B0D88C8ED4` (break `/Game/TurnBasedGame/Blueprints/Unit/Utilities/BPS_Unit_Stats` (`.Stats_8_59677AC742C58E50C0B0B8BFC3DDDE60` (break `/Game/TurnBasedGame/Blueprints/Unit/Utilities/BPS_Unit` (`self.UnitData`)))))) ShowNumber))

(fn `ModifyCurrentMp`
  (params (Modifier :type Integer) (ShowNumber :type Boolean))
  (`self.SetCurrentMp` (+ Modifier (`.MP_Current_9_342C6130430EBE8DE80D35B13735B31E` (break `/Game/TurnBasedGame/Blueprints/Unit/Utilities/BPS_Unit_Stats` (`.Stats_8_59677AC742C58E50C0B0B8BFC3DDDE60` (break `/Game/TurnBasedGame/Blueprints/Unit/Utilities/BPS_Unit` (`self.UnitData`)))))) ShowNumber))

(fn `OnSpellAnimationHit`
  (params (SpellAnimation :type "/Game/TurnBasedGame/Blueprints/Battle/Spells/BP_SpellAnims Object Reference") (TileIndex :type "IntPoint Structure"))
  (locals (SpellDamageTrue :type "/Game/TurnBasedGame/Blueprints/Battle/Spells/Utilities/BPS_SpellData_Stats_True Structure"))
  (bind (_value _returnvalue) (`BlueprintMapLibrary.Map_Find` (`self.IncomingSpells`) (`local.SpellAnimation`)))
  (if (`KismetMathLibrary.Equal_IntPointIntPoint` (`self.Index`) (`local.TileIndex`))
    (if _returnvalue :!label _label
      (set `local.SpellDamageTrue` _value)
      (`BlueprintMapLibrary.Map_Remove` (`self.IncomingSpells`) (`local.SpellAnimation`))
      (if (!= (`.Modifier_Hp_4_337387544FC677D17537229603DB65D4` (break `/Game/TurnBasedGame/Blueprints/Battle/Spells/Utilities/BPS_SpellData_Stats_True` (`local.SpellDamageTrue`))) 0)
        (`/Game/TurnBasedGame/Blueprints/Unit/Widgets/W_HpBar.UpdateHpBar` (`self.HpBar`))
        (`self.SpawnDynamicNumber` (`.Modifier_Hp_4_337387544FC677D17537229603DB65D4` (break `/Game/TurnBasedGame/Blueprints/Battle/Spells/Utilities/BPS_SpellData_Stats_True` (`local.SpellDamageTrue`))))
        (if (< (`.Modifier_Hp_4_337387544FC677D17537229603DB65D4` (break `/Game/TurnBasedGame/Blueprints/Battle/Spells/Utilities/BPS_SpellData_Stats_True` (`local.SpellDamageTrue`))) 0)
          (if (not (`self.IsAlive`))
            (if (`|EnumInequality` (`self.GetAnimationState`) "NewEnumerator4")
              (`self.SetAnimationState` "NewEnumerator4"))
            (else
              (`self.SetAnimationState` "NewEnumerator3"))))))
    (elif (`KismetMathLibrary.Equal_IntPointIntPoint` (`self.IndexDamage`) (`local.TileIndex`))
      (set `self.IndexDamage` (make `IntPoint` -999 -999))
      (goto _label))))

(fn `ResetAp`
  (`self.SetCurrentAp` (`.AP_Max_29_D6496FEF4CE2F1FA377867882D426289` (break `/Game/TurnBasedGame/Blueprints/Unit/Utilities/BPS_Unit_Stats` (`.Stats_8_59677AC742C58E50C0B0B8BFC3DDDE60` (break `/Game/TurnBasedGame/Blueprints/Unit/Utilities/BPS_Unit` (`self.UnitData`))))) true))

(fn `ResetMp`
  (`self.SetCurrentMp` (`.MP_Max_18_2725B4A5464FC373D37D05BEE793A5A3` (break `/Game/TurnBasedGame/Blueprints/Unit/Utilities/BPS_Unit_Stats` (`.Stats_8_59677AC742C58E50C0B0B8BFC3DDDE60` (break `/Game/TurnBasedGame/Blueprints/Unit/Utilities/BPS_Unit` (`self.UnitData`))))) true))

(fn `ResetUnitTotalData`
  (set `self.TotalDamageTaken` 0)
  (set `self.TotalHealingTaken` 0)
  (set `self.TotalDamageDone` 0)
  (set `self.TotalHealingDone` 0)
  (set `self.TotalSpellCast` 0)
  (set `self.TotalApSpent` 0)
  (set `self.TotalMpSpent` 0)
  (set `self.TimeAlive` 0.0)
  (set `self.TotalTurnsPerRound` 0))

(fn `SetAnimationState`
  (params (State :type "/Game/TurnBasedGame/Ressources/Units/E_StateUnitAnimation Enum" :default "NewEnumerator0"))
  (message `/Game/TurnBasedGame/Ressources/Units/BPI_UnitAnimation.SetUnitAnimationState` (`SkeletalMeshComponent.GetAnimInstance` (`self.SkeletalMesh`)) State))

(fn `SetColorByTeamIndex`
  (params (TeamIndex :type Integer))
  (set `self.TeamIndex` TeamIndex)
  (`ProgressBar.SetFillColorAndOpacity` (`/Game/TurnBasedGame/Blueprints/Unit/Widgets/W_HpBar.ProgressBar_HP` (`self.HpBar`)) (`/Game/TurnBasedGame/Blueprints/Battle/Utilities/BFL_Battle.GetTeamColor` (`self.TeamIndex`)))
  (`MeshComponent.SetVectorParameterValueOnMaterials` (`self.Mesh_TeamIndex`) "Color" (`KismetMathLibrary.Conv_LinearColorToVector` (`/Game/TurnBasedGame/Blueprints/Battle/Utilities/BFL_Battle.GetTeamColor` (`local.TeamIndex`)))))

(fn `SetCurrentAp`
  (params (Ap :type Integer) (ShowNumber :type Boolean))
  (locals (Diff :type Integer))
  (bind ((`CanMoveDiagonal_4_93F482A44F4F1FD66CC945895CDB6EDC` _canmovediagonal) (`AP_Current_28_7EC55DEC44D3AF38452837AE51007BFF` _ap_current) (`AP_Max_29_D6496FEF4CE2F1FA377867882D426289` _ap_max)) (break `/Game/TurnBasedGame/Blueprints/Unit/Utilities/BPS_Unit_Stats` (`.Stats_8_59677AC742C58E50C0B0B8BFC3DDDE60` (break `/Game/TurnBasedGame/Blueprints/Unit/Utilities/BPS_Unit` (`self.UnitData`)))))
  (bind _output_get (set `local.Diff` (- Ap _ap_current)))
  (`self.SetTotalApSpentForDebug` _output_get)
  (bind _structout (setmembers `/Game/TurnBasedGame/Blueprints/Unit/Utilities/BPS_Unit_Stats` :`StructRef` (`.Stats_8_59677AC742C58E50C0B0B8BFC3DDDE60` (break `/Game/TurnBasedGame/Blueprints/Unit/Utilities/BPS_Unit` (`self.UnitData`))) :`AP_Current` (`KismetMathLibrary.Clamp` Ap 0 _ap_max)))
  (setmembers `/Game/TurnBasedGame/Blueprints/Unit/Utilities/BPS_Unit` :`StructRef` (`self.UnitData`) :`Stats` _structout)
  (`self.OnUnitStatsChanged` self)
  (if (`local.ShowNumber`)
    (`self.SpawnDynamicNumber` (`local.Diff`) "NewEnumerator1")))

(fn `SetCurrentHp`
  (params (Hp :type Integer) (ShowNumber :type Boolean))
  (bind (_diff _clampedmax) (`self.CalculateHpDiffAndClampedMax` Hp))
  (bind _structout (setmembers `/Game/TurnBasedGame/Blueprints/Unit/Utilities/BPS_Unit_Stats` :`StructRef` (`.Stats_8_59677AC742C58E50C0B0B8BFC3DDDE60` (break `/Game/TurnBasedGame/Blueprints/Unit/Utilities/BPS_Unit` (`self.UnitData`))) :`HP_Current` _clampedmax))
  (setmembers `/Game/TurnBasedGame/Blueprints/Unit/Utilities/BPS_Unit` :`StructRef` (`self.UnitData`) :`Stats` _structout)
  (`self.OnUnitStatsChanged` self)
  ;[1 1 1] show diff in hp as animated number and notify the hp bar to update.
  (if (`local.ShowNumber`)
    (`self.SpawnDynamicNumber` _diff)
    (`/Game/TurnBasedGame/Blueprints/Unit/Widgets/W_HpBar.UpdateHpBar` (`self.HpBar`))))

(fn `SetCurrentMp`
  (params (Mp :type Integer) (ShowNumber :type Boolean))
  (bind (_diff _clampedmax) (`self.CalculateMpDiffAndClampedMax` Mp))
  (`self.SetTotalMpSpentForDebug` _diff)
  (bind _structout (setmembers `/Game/TurnBasedGame/Blueprints/Unit/Utilities/BPS_Unit_Stats` :`StructRef` (`.Stats_8_59677AC742C58E50C0B0B8BFC3DDDE60` (break `/Game/TurnBasedGame/Blueprints/Unit/Utilities/BPS_Unit` (`self.UnitData`))) :`MP_Current` _clampedmax))
  (setmembers `/Game/TurnBasedGame/Blueprints/Unit/Utilities/BPS_Unit` :`StructRef` (`self.UnitData`) :`Stats` _structout)
  (`self.OnUnitStatsChanged` self)
  ;[1 1 1] show mp spent per movement command in yellow als animated number.
  (if (`local.ShowNumber`)
    (`self.SpawnDynamicNumber` _diff "NewEnumerator2")))

(fn `SetGrid`
  (params (Grid :type "/Game/TurnBasedGame/Blueprints/Grid/BP_Grid Object Reference"))
  (bind _collision_lineofsight (`self.Collision_LineOfSight`))
  (bind _mesh_teamindex (`self.Mesh_TeamIndex`))
  (bind (_returnvalue_x _returnvalue_y _returnvalue_z) (`KismetMathLibrary.BreakVector` (`SceneComponent.K2_GetComponentScale` (`self.Collision_LineOfSight`))))
  (bind (_meshsize _mesh _meshmaterial _flatmesh _flatmaterial) (break `/Game/TurnBasedGame/Blueprints/Grid/GridRessources/BPS_DataGridShape` (`/Game/TurnBasedGame/Blueprints/Grid/BP_Grid.GetGridShapeData` (`local.Grid`))))
  (bind (_meshsize_2 _mesh_2) (break `/Game/TurnBasedGame/Blueprints/Grid/GridRessources/BPS_DataGridShape` (`/Game/TurnBasedGame/Blueprints/Grid/BP_Grid.GetGridShapeData` (`local.Grid`))))
  (bind (_returnvalue_x_2 _returnvalue_y_2) (`KismetMathLibrary.BreakVector` (/ (`/Game/TurnBasedGame/Blueprints/Grid/BP_Grid.GridTileSize` (`local.Grid`)) _meshsize_2)))
  (set `self.Grid` Grid)
  (`StaticMeshComponent.SetStaticMesh` _collision_lineofsight _mesh_2)
  (`SceneComponent.SetAbsolute` _collision_lineofsight false true true)
  (`SceneComponent.SetWorldScale3D` _collision_lineofsight (`KismetMathLibrary.MakeVector` _returnvalue_x_2 _returnvalue_y_2 _returnvalue_z))
  (`SceneComponent.K2_SetWorldRotation` _collision_lineofsight (`/Game/TurnBasedGame/Blueprints/Grid/BP_Grid.GetTileRotationFromGridIndex` (`local.Grid`) (`self.Index`)) false false)
  (`StaticMeshComponent.SetStaticMesh` _mesh_teamindex _flatmesh)
  (`PrimitiveComponent.SetMaterial` _mesh_teamindex 0 _flatmaterial)
  (`MeshComponent.SetScalarParameterValueOnMaterials` _mesh_teamindex "IsFilled" 1.0)
  (`SceneComponent.SetAbsolute` _mesh_teamindex false true true)
  (`SceneComponent.SetWorldScale3D` _mesh_teamindex (/ (`/Game/TurnBasedGame/Blueprints/Grid/BP_Grid.GridTileSize` (`local.Grid`)) _meshsize))
  (`SceneComponent.K2_SetWorldRotation` _mesh_teamindex (`/Game/TurnBasedGame/Blueprints/Grid/BP_Grid.GetTileRotationFromGridIndex` (`local.Grid`) (`self.Index`)) false false)
  (`SceneComponent.K2_SetRelativeLocation` _mesh_teamindex (`KismetMathLibrary.MakeVector` 0.0 0.0 (+ (`/Game/TurnBasedGame/Blueprints/Grid/Utilities/BP_GridVisible.OffsetFromGround` (`/Game/TurnBasedGame/Blueprints/Grid/BP_Grid.GridVisual` (`local.Grid`))) 5.0)) false false))

(fn `SetGridIndex`
  (params (Index :type "IntPoint Structure"))
  (set `self.Index` Index)
  (`SceneComponent.K2_SetWorldRotation` (`self.Collision_LineOfSight`) (`/Game/TurnBasedGame/Blueprints/Grid/BP_Grid.GetTileRotationFromGridIndex` (`self.Grid`) (`local.Index`)) false false)
  (`SceneComponent.K2_SetWorldRotation` (`self.Mesh_TeamIndex`) (`/Game/TurnBasedGame/Blueprints/Grid/BP_Grid.GetTileRotationFromGridIndex` (`self.Grid`) (`local.Index`)) false false))

(fn `SetIsHovered`
  (params (Hovered :type Boolean))
  (set `self.IsHovered` Hovered)
  (`self.UpdateColorSelectedHoveredUnit`)
  (`self.OnUnitHoveredChanged` self))

(fn `SetIsInBattle`
  (params (IsInBattle :type Boolean))
  (set `self.IsInBattle` IsInBattle)
  (`self.UpdateColorSelectedHoveredUnit`)
  (`self.OnUnitIsInBattleChanged` self))

(fn `SetIsSelected`
  (params (Selected :type Boolean))
  (set `self.IsSelected` Selected)
  (`self.UpdateColorSelectedHoveredUnit`)
  (`self.OnUnitSelectedChanged` self))

(fn `SetNextTransformLocation`
  (bind _previoustransform_location (`KismetMathLibrary.BreakTransform` (`self.PreviousTransform`)))
  (bind (_index _type _transform) (break `/Game/TurnBasedGame/Blueprints/Grid/Utilities/BPS_DataTile` (`BlueprintMapLibrary.Map_Find` (`/Game/TurnBasedGame/Blueprints/Grid/BP_Grid.GridTiles` (`self.Grid`)) (`|GetArrayItem` (`self.CurrentPathToFollow`)))))
  (bind (_returnvalue_roll _returnvalue_pitch _returnvalue_yaw) (`KismetMathLibrary.BreakRotator` (`KismetMathLibrary.FindLookAtRotation` _previoustransform_location (.location _transform))))
  (set `self.NextTransform` (`KismetMathLibrary.MakeTransform` (.location _transform) (`KismetMathLibrary.MakeRotator` 0.0 0.0 _returnvalue_yaw))))

(fn `SetTotalApSpentForDebug`
  (params (A :type Integer))
  (if (> A 0)
    (set `self.TotalApSpent` (+ (`self.TotalApSpent`) A))))

(fn `SetTotalDamageAndHealingTakenForDebug`
  (params (Dif :type Integer))
  (if (> Dif 0)
    (set `self.TotalHealingTaken` (+ (`self.TotalHealingTaken`) Dif))
    (else
      (set `self.TotalDamageTaken` (- (`self.TotalDamageTaken`) Dif)))))

(fn `SetTotalMpSpentForDebug`
  (params (Diff :type Integer))
  (if (> Diff 0)
    (set `self.TotalMpSpent` (+ (`self.TotalMpSpent`) Diff))))

(fn `SetUnitAI`
  (params (AI :type "/Game/TurnBasedGame/Blueprints/AI/BP_AI Object Reference"))
  (bind _output_get (set `self.AI` AI))
  (`/Engine/EditorBlueprintResources/StandardMacros.IsValid` _output_get
    (:`Is Valid`
      (`self.K2_AttachToActor` (`local.AI`) self "None" "SnapToTarget" "SnapToTarget" "SnapToTarget" true))))

(fn `SetUnitData`
  (params (Data :type "/Game/TurnBasedGame/Blueprints/Unit/Utilities/BPS_Unit Structure (by ref)"))
  (bind _skeletalmesh (`self.SkeletalMesh`))
  (bind _hpbar (`self.HpBar`))
  ;[1 1 1] sets mesh and animation of the unit as defined in given data.
  (bind _output_get (set `self.UnitData` Data))
  (bind (_mesh _icon _animation) (break `/Game/TurnBasedGame/Blueprints/Unit/Utilities/BPS_Unit_Assets` (`.Assets_5_FC045E6540DEB6F3C40A4DBF44D686F8` (break `/Game/TurnBasedGame/Blueprints/Unit/Utilities/BPS_Unit` _output_get))))
  (`SkeletalMeshComponent.SetSkeletalMeshAsset` _skeletalmesh _mesh)
  (`SkeletalMeshComponent.SetAnimInstanceClass` _skeletalmesh _animation)
  ;[1 1 1] update the hp bar if stats change, mainly hp. only do this if hpbar is valid (unit not dead).
  (`self.OnUnitStatsChanged` self)
  (`/Engine/EditorBlueprintResources/StandardMacros.IsValid` _hpbar
    (:`Is Valid`
      (`/Game/TurnBasedGame/Blueprints/Unit/Widgets/W_HpBar.UpdateHpBar` _hpbar))))

(fn `SpawnDynamicNumber`
  (params (Number :type Integer) (Color :type "/Game/TurnBasedGame/Blueprints/Unit/Widgets/BPE_DynamicNumber_Colors Enum" :default "NewEnumerator0"))
  (if (!= Number 0)
    (`|SpawnActorFromClass` "/Game/TurnBasedGame/Blueprints/Unit/Widgets/BP_DynamicNumber.BP_DynamicNumber_C" (`KismetMathLibrary.MakeTransform` (`self.K2_GetActorLocation`)) "Undefined" "MultiplyWithRoot" null Number Color null)))

(fn `TurnEnded`
  (`self.SetIsInBattle` false)
  (if (`self.IsAlive`)
    (`self.ResetMp`)
    (`self.ResetAp`)))

(fn `TurnStarted`
  ;[1 1 1] used to calculate turns per round per unit.
  (set `self.TotalTurnsPerRound` (+ (`self.TotalTurnsPerRound`) 1))
  (`self.SetIsInBattle` true))

(fn `UpdateColorSelectedHoveredUnit`
  (`MeshComponent.SetVectorParameterValueOnMaterials` (`self.SkeletalMesh`) "ColorMultiply" (`KismetMathLibrary.Conv_LinearColorToVector` (* (* (`KismetMathLibrary.SelectColor` (struct :`R` 1.0 :`G` 0.862745 :`B` 0.090196 :`A` 1.0) (struct :`R` 1.0 :`G` 1.0 :`B` 1.0 :`A` 1.0) (or (`self.IsSelected`) (`self.IsInBattle`))) (`KismetMathLibrary.SelectFloat` 1.0 2.5 (not (`self.IsHovered`)))) (`KismetMathLibrary.SelectFloat` 1.0 2.5 (not (or (`self.IsSelected`) (`self.IsInBattle`))))))))

(fn `UserConstructionScript`
  (bind _unitdata (`/Game/TurnBasedGame/Blueprints/Unit/Utilities/BFL_Units.GetDefaultUnitDataFromUnitType` (`self.UnitType`)))
  (`self.SetUnitData` _unitdata))