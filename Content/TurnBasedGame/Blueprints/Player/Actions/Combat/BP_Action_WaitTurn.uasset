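; Wait-turn combat action for the turn-based grid game that, as shown here, previews the tiles a unit can reach with its current movement points.
; On hover it targets the hovered unit, falling back to the selected one, and recalculates only when that unit changes.
; A time-budgeted grid pathfinder uses the unit's movement stats, and its completion callback marks reachable tiles.
; Tile marks clear on unit change and EndPlay.
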(event `self.ReceiveBeginPlay`
  (`parent.ReceiveBeginPlay`)
  (add `/Game/TurnBasedGame/Blueprints/Grid/BP_Pathfinding.OnPathfindingCompleted` (`/Game/TurnBasedGame/Blueprints/Grid/BP_Grid.GridPathfinding_ReachableTile` (`/Game/TurnBasedGame/Blueprints/Player/BP_PlayerActions.Grid` (`self.PlayerActions`))) (`|CreateDelegate` :!event `OnPathfindingCompleted_Reachables`)))

(event `self.ReceiveEndPlay`
  (params (EndPlayReason :type "EEndPlayReason Enum" :default "Destroyed"))
  (`parent.ReceiveEndPlay` EndPlayReason)
  (`/Game/TurnBasedGame/Blueprints/Grid/BP_Grid.ClearStateFromTiles` (`/Game/TurnBasedGame/Blueprints/Player/BP_PlayerActions.Grid` (`self.PlayerActions`)) "NewEnumerator7"))

(fn `CalculateReachableTilesForCurrentUnit`
  (params (Target :type "/Game/TurnBasedGame/Blueprints/Units/BP_Unit Object Reference"))
  (returns (Path :type "Array of IntPoint Structure"))
  (bind ((`ValidTileTypes_6_15FC62644524545BA5E30EA063EF24D4` _validtiletypes) (`CanMoveDiagonal_4_93F482A44F4F1FD66CC945895CDB6EDC` _canmovediagonal) (`MP_Current_9_342C6130430EBE8DE80D35B13735B31E` _mp_current)) (break `/Game/TurnBasedGame/Blueprints/Units/Utilities/BPS_Unit_Stats` (`.Stats_8_59677AC742C58E50C0B0B8BFC3DDDE60` (break `/Game/TurnBasedGame/Blueprints/Units/Utilities/BPS_Unit` (`/Game/TurnBasedGame/Blueprints/Units/BP_Unit.UnitData` Target)))))
  (bind _path (`/Game/TurnBasedGame/Blueprints/Grid/BP_Pathfinding.FindPath` :`self` (`/Game/TurnBasedGame/Blueprints/Grid/BP_Grid.GridPathfinding_ReachableTile` (`/Game/TurnBasedGame/Blueprints/Player/BP_PlayerActions.Grid` (`self.PlayerActions`))) :`Start` (`/Game/TurnBasedGame/Blueprints/Units/BP_Unit.Index` Target) :`Diagonals` _canmovediagonal :`TileTypes` _validtiletypes :`Delay` 0.1 :`MaxMs` 15.0 :`ReturnReachables` true :`PathLength` _mp_current))
  (return _path))

(fn `ExecuteHoveredAction`
  (params (Index :type "IntPoint Structure"))
  (bind _playeractions (`self.PlayerActions`))
  (bind _hoveredunit (`/Game/TurnBasedGame/Blueprints/Player/BP_PlayerActions.HoveredUnit` _playeractions))
  (`parent.ExecuteHoveredAction` Index)
  (`/Engine/EditorBlueprintResources/StandardMacros.IsValid` _hoveredunit
    (:`Is Valid`
      (`self.GenerateReachableTiles` _hoveredunit))
    (:`Is Not Valid`
      (`self.GenerateReachableTiles` (`/Game/TurnBasedGame/Blueprints/Player/BP_PlayerActions.SelectedUnit` _playeractions)))))

(fn `GenerateReachableTiles`
  (params (Unit :type "/Game/TurnBasedGame/Blueprints/Units/BP_Unit Object Reference"))
  (bind _currentunitforreachables (`self.CurrentUnitForReachables`))
  (if (!= Unit (`self.CurrentUnitForReachables`))
    (set `self.CurrentUnitForReachables` Unit)
    (`/Game/TurnBasedGame/Blueprints/Grid/BP_Grid.ClearStateFromTiles` (`/Game/TurnBasedGame/Blueprints/Player/BP_PlayerActions.Grid` (`self.PlayerActions`)) "NewEnumerator7")
    (`/Engine/EditorBlueprintResources/StandardMacros.IsValid` _currentunitforreachables
      (:`Is Valid`
        (`self.CalculateReachableTilesForCurrentUnit` _currentunitforreachables)))))

(fn `OnPathfindingCompleted_Reachables`
  (params (Reachables :type "Array of IntPoint Structure"))
  (for _array_element Reachables
    (`/Game/TurnBasedGame/Blueprints/Grid/BP_Grid.AddStateToTile` (`/Game/TurnBasedGame/Blueprints/Player/BP_PlayerActions.Grid` (`self.PlayerActions`)) _array_element "NewEnumerator7")))

(fn `UserConstructionScript`
  (`parent.UserConstructionScript`))