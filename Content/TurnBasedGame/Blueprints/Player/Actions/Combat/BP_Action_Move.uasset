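; Combat move action for a turn-based grid game that previews and executes movement of the selected unit.
; Hovering highlights reachable tiles for the hovered or selected unit, plus a path to the hovered tile when no unit is there.
; Two grid pathfinding components report via completion events, using the unit's movement stats.
; Executing passes the stored path to the combat system, and walk start/finish events pause and refresh previews.
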(event `self.ReceiveBeginPlay`
  (bind _selectedunit (`/Game/TurnBasedGame/Blueprints/Player/BP_PlayerActions.SelectedUnit` (`self.PlayerActions`)))
  (`parent.ReceiveBeginPlay`)
  (add `/Game/TurnBasedGame/Blueprints/Grid/BP_Pathfinding.OnPathfindingCompleted` (`/Game/TurnBasedGame/Blueprints/Grid/BP_Grid.GridPathfinding_ReachableTile` (`/Game/TurnBasedGame/Blueprints/Player/BP_PlayerActions.Grid` (`self.PlayerActions`))) (`|CreateDelegate` :!event `OnPathfindingCompleted_Reachables`))
  (add `/Game/TurnBasedGame/Blueprints/Grid/BP_Pathfinding.OnPathfindingCompleted` (`/Game/TurnBasedGame/Blueprints/Grid/BP_Grid.GridPathfinding` (`/Game/TurnBasedGame/Blueprints/Player/BP_PlayerActions.Grid` (`self.PlayerActions`))) (`|CreateDelegate` :!event `OnPathfindingCompleted_Path`))
  (add `/Game/TurnBasedGame/Blueprints/Units/BP_Unit.OnUnitStartedWalking` _selectedunit (`|CreateDelegate` :!event `OnUnitStartedWalking`))
  (add `/Game/TurnBasedGame/Blueprints/Units/BP_Unit.OnUnitFinishedWalking` _selectedunit (`|CreateDelegate` :!event `OnUnitFinishedWalking`))
  (`self.GenerateReachables` (`/Game/TurnBasedGame/Blueprints/Player/BP_PlayerActions.SelectedUnit` (`self.PlayerActions`))))

(event `self.ReceiveEndPlay`
  (params (EndPlayReason :type "EEndPlayReason Enum" :default "Destroyed"))
  (bind _grid (`/Game/TurnBasedGame/Blueprints/Player/BP_PlayerActions.Grid` (`self.PlayerActions`)))
  (`parent.ReceiveEndPlay` EndPlayReason)
  (`/Game/TurnBasedGame/Blueprints/Grid/BP_Grid.ClearStateFromTiles` _grid "NewEnumerator7")
  (`/Game/TurnBasedGame/Blueprints/Grid/BP_Grid.ClearStateFromTiles` _grid "NewEnumerator4"))

(fn `CalculatePathForGivenTarget`
  (params (Target :type "/Game/TurnBasedGame/Blueprints/Units/BP_Unit Object Reference") (ReturnReachables :type Boolean) (Tile :type "IntPoint Structure") (Pathfinding :type "/Game/TurnBasedGame/Blueprints/Grid/BP_Pathfinding Object Reference"))
  (bind ((`ValidTileTypes_6_15FC62644524545BA5E30EA063EF24D4` _validtiletypes) (`CanMoveDiagonal_4_93F482A44F4F1FD66CC945895CDB6EDC` _canmovediagonal) (`MP_Current_9_342C6130430EBE8DE80D35B13735B31E` _mp_current)) (break `/Game/TurnBasedGame/Blueprints/Units/Utilities/BPS_Unit_Stats` (`.Stats_8_59677AC742C58E50C0B0B8BFC3DDDE60` (break `/Game/TurnBasedGame/Blueprints/Units/Utilities/BPS_Unit` (`/Game/TurnBasedGame/Blueprints/Units/BP_Unit.UnitData` Target)))))
  (`/Game/TurnBasedGame/Blueprints/Grid/BP_Pathfinding.FindPath` Pathfinding (`/Game/TurnBasedGame/Blueprints/Units/BP_Unit.Index` Target) Tile _canmovediagonal _validtiletypes 0.1 15.0 ReturnReachables _mp_current))

(fn `ExecuteAction`
  (params (Index :type "IntPoint Structure"))
  (bind _playeractions (`self.PlayerActions`))
  (`parent.ExecuteAction` Index)
  (if (> (`KismetArrayLibrary.Array_Length` (`self.GeneratedPath`)) 0)
    (`/Game/TurnBasedGame/Blueprints/Combat/BP_Combat.MoveUnit` (`/Game/TurnBasedGame/Blueprints/Player/BP_PlayerActions.CombatSystem` _playeractions) (`/Game/TurnBasedGame/Blueprints/Player/BP_PlayerActions.SelectedUnit` _playeractions) (`self.GeneratedPath`))
    (`KismetArrayLibrary.Array_Clear` (`self.GeneratedPath`))))

(fn `ExecuteHoveredAction`
  (params (Index :type "IntPoint Structure"))
  (bind _playeractions (`self.PlayerActions`))
  (bind _hoveredunit (`/Game/TurnBasedGame/Blueprints/Player/BP_PlayerActions.HoveredUnit` _playeractions))
  (`parent.ExecuteHoveredAction` Index)
  (if (not (`self.IsUnitWalking`))
    ;[1 1 1] only generate the actual path for selected units. show reachable tiles for hovered units.
    (`/Engine/EditorBlueprintResources/StandardMacros.IsValid` _hoveredunit
      (:`Is Valid`
        (`self.GenerateReachables` _hoveredunit))
      (:`Is Not Valid`
        (`self.GenerateReachables` (`/Game/TurnBasedGame/Blueprints/Player/BP_PlayerActions.SelectedUnit` _playeractions))
        (`self.GeneratePath`)))))

(fn `GeneratePath`
  (bind _playeractions (`self.PlayerActions`))
  (`/Game/TurnBasedGame/Blueprints/Grid/BP_Grid.ClearStateFromTiles` (`/Game/TurnBasedGame/Blueprints/Player/BP_PlayerActions.Grid` (`self.PlayerActions`)) "NewEnumerator4")
  (`KismetArrayLibrary.Array_Clear` (`self.GeneratedPath`))
  (`self.CalculatePathForGivenTarget` (`/Game/TurnBasedGame/Blueprints/Player/BP_PlayerActions.SelectedUnit` _playeractions) false (`/Game/TurnBasedGame/Blueprints/Player/BP_PlayerActions.HoveredTile` _playeractions) (`/Game/TurnBasedGame/Blueprints/Grid/BP_Grid.GridPathfinding` (`/Game/TurnBasedGame/Blueprints/Player/BP_PlayerActions.Grid` _playeractions))))

(fn `GenerateReachables`
  (params (Unit :type "/Game/TurnBasedGame/Blueprints/Units/BP_Unit Object Reference"))
  (bind _playeractions (`self.PlayerActions`))
  (if (!= Unit (`self.CurrentUnitForReachables`))
    (set `self.CurrentUnitForReachables` Unit)
    (`/Game/TurnBasedGame/Blueprints/Grid/BP_Grid.ClearStateFromTiles` (`/Game/TurnBasedGame/Blueprints/Player/BP_PlayerActions.Grid` _playeractions) "NewEnumerator7")
    (`self.CalculatePathForGivenTarget` (`self.CurrentUnitForReachables`) true (struct) (`/Game/TurnBasedGame/Blueprints/Grid/BP_Grid.GridPathfinding_ReachableTile` (`/Game/TurnBasedGame/Blueprints/Player/BP_PlayerActions.Grid` _playeractions)))))

(fn `OnPathfindingCompleted_Path`
  (params (Path :type "Array of IntPoint Structure"))
  (bind _output_get (set `self.GeneratedPath` Path))
  (for _array_element _output_get
    (`/Game/TurnBasedGame/Blueprints/Grid/BP_Grid.AddStateToTile` (`/Game/TurnBasedGame/Blueprints/Player/BP_PlayerActions.Grid` (`self.PlayerActions`)) _array_element "NewEnumerator4")))

(fn `OnPathfindingCompleted_Reachables`
  (params (Reachables :type "Array of IntPoint Structure"))
  (if (not (`self.IsUnitWalking`))
    (for _array_element Reachables
      (`/Game/TurnBasedGame/Blueprints/Grid/BP_Grid.AddStateToTile` (`/Game/TurnBasedGame/Blueprints/Player/BP_PlayerActions.Grid` (`self.PlayerActions`)) _array_element "NewEnumerator7"))))

(fn `OnUnitFinishedWalking`
  (params (Unit :type "/Game/TurnBasedGame/Blueprints/Units/BP_Unit Object Reference"))
  (set `self.IsUnitWalking` false)
  (`self.ExecuteHoveredAction` (`/Game/TurnBasedGame/Blueprints/Player/BP_PlayerActions.HoveredTile` (`self.PlayerActions`))))

(fn `OnUnitStartedWalking`
  (params (Unit :type "/Game/TurnBasedGame/Blueprints/Units/BP_Unit Object Reference"))
  (set `self.IsUnitWalking` true)
  (`/Game/TurnBasedGame/Blueprints/Grid/BP_Grid.ClearStateFromTiles` (`/Game/TurnBasedGame/Blueprints/Player/BP_PlayerActions.Grid` (`self.PlayerActions`)) "NewEnumerator7")
  (set `self.CurrentUnitForReachables` null))

(fn `UserConstructionScript`
  (`parent.UserConstructionScript`))