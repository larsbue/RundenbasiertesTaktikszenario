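; Player action for the turn-based grid that finds and highlights a path from the selected tile to a target index.
; Executing it clears previous path states and calls GridPathfinding with options for diagonals, flying-only tiles, max length and iteration delay or per-frame time budget.
; A completion callback marks each returned tile as in-path to update visuals.
; Selection changes and EndPlay re-run it with an out-of-range index, clearing the path.
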(event `self.ReceiveBeginPlay`
  (add `/Game/TurnBasedGame/Blueprints/Player/BP_PlayerActions.OnSelectedTilesChanged` (`self.PlayerActions`) (delegate `OnSelectedTileChanged`)))

(event `OnSelectedTileChanged`
  (params (Index :type "IntPoint Structure"))
  (`self.ExecuteAction` (make `IntPoint` -999 -999)))

(event `self.ReceiveEndPlay`
  (params (EndPlayReason :type "EEndPlayReason Enum" :default "Destroyed"))
  (`self.ExecuteAction` (make `IntPoint` -999 -999)))

(fn `CalculatePathWithCostFactors`
  (`/Game/TurnBasedGame/Blueprints/Grid/BP_Pathfinding.FindPath` (`/Game/TurnBasedGame/Blueprints/Grid/BP_Grid.GridPathfinding` (`/Game/TurnBasedGame/Blueprints/Player/BP_PlayerActions.Grid` (`self.PlayerActions`))) (`/Game/TurnBasedGame/Blueprints/Player/BP_PlayerActions.SelectedTile` (`self.PlayerActions`)) (`self.Index`) (`self.IncludeDiagonals`) (select `bool` (`self.IncludeFlyingOnly`) :`false` (`|MakeArray` "NewEnumerator1" "NewEnumerator3" "NewEnumerator4" :!type "/Game/TurnBasedGame/Blueprints/Grid/Utilities/BPE_TypeTile Enum") :`true` (`|MakeArray` "NewEnumerator1" "NewEnumerator3" "NewEnumerator4" "NewEnumerator5" :!type "/Game/TurnBasedGame/Blueprints/Grid/Utilities/BPE_TypeTile Enum")) (`self.DelayBetweenIterations`) (`self.MaxMsPerFrame`) false (`self.MaxPathLength`)))

(fn `ExecuteAction`
  (params (Index :type "IntPoint Structure"))
  (set `self.Index` Index)
  ;[1 1 1] first, clear all states from tiles in path.
  (`/Game/TurnBasedGame/Blueprints/Grid/BP_Grid.ClearStateFromTiles` (`/Game/TurnBasedGame/Blueprints/Player/BP_PlayerActions.Grid` (`self.PlayerActions`)) "NewEnumerator4")
  ;[1 1 1] create event and transmit calculated path
  (add `/Game/TurnBasedGame/Blueprints/Grid/BP_Pathfinding.OnPathfindingCompleted` (`/Game/TurnBasedGame/Blueprints/Grid/BP_Grid.GridPathfinding` (`/Game/TurnBasedGame/Blueprints/Player/BP_PlayerActions.Grid` (`self.PlayerActions`))) (`|CreateDelegate` :!event `OnPathfindingCompleted`))
  (`self.CalculatePathWithCostFactors`))

(fn `OnPathfindingCompleted`
  (params (Path :type "Array of IntPoint Structure"))
  ;[1 1 1] iterates over all tiles in a path to mark every tile on route with IsInPath-State (to update the visuals of the path)
  (for _array_element Path
    (`/Game/TurnBasedGame/Blueprints/Grid/BP_Grid.AddStateToTile` (`/Game/TurnBasedGame/Blueprints/Player/BP_PlayerActions.Grid` (`self.PlayerActions`)) _array_element "NewEnumerator4")))

(fn `UserConstructionScript`
  (`parent.UserConstructionScript`))