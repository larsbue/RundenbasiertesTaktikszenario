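; Player action that moves the selected unit along a calculated grid path toward a target tile in the turn-based game.
; Executing it clears old path tiles, binds to pathfinding and walk-finished events, then requests a path using the unit's movement stats.
; The completed path is highlighted, walked through Battle, followed by an MP reset; highlights clear when walking ends.
; EndPlay re-executes with an out-of-range index.
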(event `self.ReceiveEndPlay`
  (params (EndPlayReason :type "EEndPlayReason Enum" :default "Destroyed"))
  (`self.ExecuteAction` (make `IntPoint` -999 -999)))

(fn `CalculatePathForGivenUnit`
  (bind (_validtiletypes _canmovediagonal _hp_current _hp_max _mp_current) (break `/Game/TurnBasedGame/Blueprints/Unit/Utilities/BPS_Unit_Stats` (`.Stats_8_59677AC742C58E50C0B0B8BFC3DDDE60` (break `/Game/TurnBasedGame/Blueprints/Unit/Utilities/BPS_Unit` (`/Game/TurnBasedGame/Blueprints/Unit/BP_Unit.UnitData` (`self.CurrentUnit`))))))
  (`/Game/TurnBasedGame/Blueprints/Grid/BP_Pathfinding.FindPath` (`/Game/TurnBasedGame/Blueprints/Grid/BP_Grid.GridPathfinding` (`/Game/TurnBasedGame/Blueprints/Player/BP_PlayerActions.Grid` (`self.PlayerActions`))) (`/Game/TurnBasedGame/Blueprints/Player/BP_PlayerActions.SelectedTile` (`self.PlayerActions`)) (`self.Index`) _canmovediagonal _validtiletypes 0.0 0.0 false _mp_current))

(fn `ExecuteAction`
  (params (Index :type "IntPoint Structure"))
  (set `self.Index` Index)
  (`/Game/TurnBasedGame/Blueprints/Grid/BP_Grid.ClearStateFromTiles` (`/Game/TurnBasedGame/Blueprints/Player/BP_PlayerActions.Grid` (`self.PlayerActions`)) "NewEnumerator4")
  (bind _output_get (set `self.CurrentUnit` (`/Game/TurnBasedGame/Blueprints/Player/BP_PlayerActions.SelectedUnit` (`self.PlayerActions`))))
  (`/Engine/EditorBlueprintResources/StandardMacros.IsValid` _output_get
    (:`Is Valid`
      ;[1 1 1] create event after unit is finished walking to clear states from tiles in path.
      (add `/Game/TurnBasedGame/Blueprints/Unit/BP_Unit.OnUnitFinishedWalking` (`self.CurrentUnit`) (`|CreateDelegate` :!event `OnUnitFinishedWalking`))
      ;;[1 1 1] create event after path is calculated.
      (add `/Game/TurnBasedGame/Blueprints/Grid/BP_Pathfinding.OnPathfindingCompleted` (`/Game/TurnBasedGame/Blueprints/Grid/BP_Grid.GridPathfinding` (`/Game/TurnBasedGame/Blueprints/Player/BP_PlayerActions.Grid` (`self.PlayerActions`))) (`|CreateDelegate` :!event `OnPathfindingCompleted`))
      (`self.CalculatePathForGivenUnit`))))

(fn `OnPathfindingCompleted`
  (params (Path :type "Array of IntPoint Structure"))
  (`/Engine/EditorBlueprintResources/StandardMacros.IsValid` (`self.CurrentUnit`)
    (:`Is Valid`
      (if (== (`self.CurrentUnit`) (`/Game/TurnBasedGame/Blueprints/Player/BP_PlayerActions.SelectedUnit` (`self.PlayerActions`)))
        ;[1 1 1] add IsInPath state to every tile of the path to visually showcase it.
        (for _array_element (`local.Path`)
          (`/Game/TurnBasedGame/Blueprints/Grid/BP_Grid.AddStateToTile` (`/Game/TurnBasedGame/Blueprints/Player/BP_PlayerActions.Grid` (`self.PlayerActions`)) _array_element "NewEnumerator4"))
        ;[1 1 1] after all states have been added to the tiles in path, move the unit on the calculated path and reset the movementpoints.
        (set `/Game/TurnBasedGame/Blueprints/Unit/BP_Unit.MoveDurationPerTile` (`self.MoveDuration`) (`self.CurrentUnit`))
        (`/Game/TurnBasedGame/Blueprints/Battle/BP_Battle.MoveUnit` (`/Game/TurnBasedGame/Blueprints/Player/BP_PlayerActions.Battle` (`self.PlayerActions`)) (`self.CurrentUnit`) (`local.Path`))
        (`/Game/TurnBasedGame/Blueprints/Unit/BP_Unit.ResetMp` (`self.CurrentUnit`))))))

(fn `OnUnitFinishedWalking`
  (params (Unit :type "/Game/TurnBasedGame/Blueprints/Unit/BP_Unit Object Reference"))
  (if (== Unit (`self.CurrentUnit`))
    (`/Game/TurnBasedGame/Blueprints/Grid/BP_Grid.ClearStateFromTiles` (`/Game/TurnBasedGame/Blueprints/Player/BP_PlayerActions.Grid` (`self.PlayerActions`)) "NewEnumerator4")))

(fn `UserConstructionScript`
  (`parent.UserConstructionScript`))