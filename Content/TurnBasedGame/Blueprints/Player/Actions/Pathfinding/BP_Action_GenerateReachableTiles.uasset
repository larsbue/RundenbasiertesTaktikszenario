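; Player action that highlights the tiles reachable from the selected tile on the turn-based grid.
; It runs the grid's reachable-tile pathfinder in return-reachables mode and applies a tile state to the results on completion.
; A selected unit supplies diagonal movement, valid tile types and current MP; otherwise the action's own settings apply, including iteration delay and per-frame budget.
; Highlights clear when that unit starts walking and regenerate when it finishes.
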(fn `CalculateReachableTilesWithSelectedTile`
  (`/Game/TurnBasedGame/Blueprints/Grid/BP_Pathfinding.FindPath` (`/Game/TurnBasedGame/Blueprints/Grid/BP_Grid.GridPathfinding_ReachableTile` (`/Game/TurnBasedGame/Blueprints/Player/BP_PlayerActions.Grid` (`self.PlayerActions`))) (`/Game/TurnBasedGame/Blueprints/Player/BP_PlayerActions.SelectedTile` (`self.PlayerActions`)) (make `IntPoint` -999 -999) (`self.IncludeDiagonals`) (select `bool` (`self.IncludeFlyingOnly`) :`false` (`|MakeArray` "NewEnumerator1" "NewEnumerator3" "NewEnumerator4" :!type "/Game/TurnBasedGame/Blueprints/Grid/Utilities/BPE_TypeTile Enum") :`true` (`|MakeArray` "NewEnumerator1" "NewEnumerator3" "NewEnumerator4" "NewEnumerator5" :!type "/Game/TurnBasedGame/Blueprints/Grid/Utilities/BPE_TypeTile Enum")) (`self.DelayBetweenIterations`) (`self.MaxMsPerFrame`) true (`self.MaxPathLength`)))

(fn `CalculateReachableTilesWithUnitData`
  (bind (_validtiletypes _canmovediagonal _hp_current _hp_max _mp_current) (break `/Game/TurnBasedGame/Blueprints/Unit/Utilities/BPS_Unit_Stats` (`.Stats_8_59677AC742C58E50C0B0B8BFC3DDDE60` (break `/Game/TurnBasedGame/Blueprints/Unit/Utilities/BPS_Unit` (`/Game/TurnBasedGame/Blueprints/Unit/BP_Unit.UnitData` (`/Game/TurnBasedGame/Blueprints/Player/BP_PlayerActions.SelectedUnit` (`self.PlayerActions`)))))))
  (`/Game/TurnBasedGame/Blueprints/Grid/BP_Pathfinding.FindPath` (`/Game/TurnBasedGame/Blueprints/Grid/BP_Grid.GridPathfinding_ReachableTile` (`/Game/TurnBasedGame/Blueprints/Player/BP_PlayerActions.Grid` (`self.PlayerActions`))) (`/Game/TurnBasedGame/Blueprints/Player/BP_PlayerActions.SelectedTile` (`self.PlayerActions`)) (make `IntPoint` -999 -999) _canmovediagonal _validtiletypes 0.0 0.0 true _mp_current))

(fn `ExecuteAction`
  (params (Index :type "IntPoint Structure"))
  (`parent.ExecuteAction` Index)
  (`self.GenerateReachableTiles`))

(fn `GenerateReachableTiles`
  (bind _selectedunit (`/Game/TurnBasedGame/Blueprints/Player/BP_PlayerActions.SelectedUnit` (`self.PlayerActions`)))
  (`/Game/TurnBasedGame/Blueprints/Grid/BP_Grid.ClearStateFromTiles` (`/Game/TurnBasedGame/Blueprints/Player/BP_PlayerActions.Grid` (`self.PlayerActions`)) "NewEnumerator7")
  (add `/Game/TurnBasedGame/Blueprints/Grid/BP_Pathfinding.OnPathfindingCompleted` (`/Game/TurnBasedGame/Blueprints/Grid/BP_Grid.GridPathfinding_ReachableTile` (`/Game/TurnBasedGame/Blueprints/Player/BP_PlayerActions.Grid` (`self.PlayerActions`))) (`|CreateDelegate` :!event `OnPathfindingCompleted`))
  ;[1 1 1] if no unit selected, generate reachable tiles from selected tile.
  (`/Engine/EditorBlueprintResources/StandardMacros.IsValid` (`/Game/TurnBasedGame/Blueprints/Player/BP_PlayerActions.SelectedUnit` (`self.PlayerActions`))
    (:`Is Valid`
      (add `/Game/TurnBasedGame/Blueprints/Unit/BP_Unit.OnUnitStartedWalking` _selectedunit (`|CreateDelegate` :!event `OnUnitStartedWalking`))
      (add `/Game/TurnBasedGame/Blueprints/Unit/BP_Unit.OnUnitFinishedWalking` _selectedunit (`|CreateDelegate` :!event `OnUnitFinishedWalking`))
      (`self.CalculateReachableTilesWithUnitData`))
    (:`Is Not Valid`
      (`self.CalculateReachableTilesWithSelectedTile`))))

(fn `OnPathfindingCompleted`
  (params (Path :type "Array of IntPoint Structure (by ref)"))
  (for _array_element Path
    (`/Game/TurnBasedGame/Blueprints/Grid/BP_Grid.AddStateToTile` (`/Game/TurnBasedGame/Blueprints/Player/BP_PlayerActions.Grid` (`self.PlayerActions`)) _array_element "NewEnumerator7")))

(fn `OnUnitFinishedWalking`
  (params (Unit :type "/Game/TurnBasedGame/Blueprints/Unit/BP_Unit Object Reference"))
  (`self.GenerateReachableTiles`))

(fn `OnUnitStartedWalking`
  (params (Unit :type "/Game/TurnBasedGame/Blueprints/Unit/BP_Unit Object Reference"))
  (`/Game/TurnBasedGame/Blueprints/Grid/BP_Grid.ClearStateFromTiles` (`/Game/TurnBasedGame/Blueprints/Player/BP_PlayerActions.Grid` (`self.PlayerActions`)) "NewEnumerator7"))

(fn `UserConstructionScript`
  (`parent.UserConstructionScript`))