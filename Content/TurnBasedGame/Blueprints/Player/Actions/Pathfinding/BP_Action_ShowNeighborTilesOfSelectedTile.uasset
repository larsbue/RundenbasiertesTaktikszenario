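; Player action that highlights the valid neighbors of a selected tile on the turn-based game's grid.
; ExecuteAction clears the IsNeighbor state, asks GridPathfinding for valid neighbors, optionally including diagonals and filtered by allowed tile types, then adds the state to each.
; EndPlay re-runs the action with an off-grid sentinel index, clearing the highlights when the action ends.
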(event `self.ReceiveEndPlay`
  (params (EndPlayReason :type "EEndPlayReason Enum" :default "Destroyed"))
  (`self.ExecuteAction` (make `IntPoint` -999 -999)))

(fn `ExecuteAction`
  (params (Index :type "IntPoint Structure"))
  ;[1 1 1] as usual, clear all IsNeigbor states from tiles so we can see new ones.
  (`/Game/TurnBasedGame/Blueprints/Grid/BP_Grid.ClearStateFromTiles` (`/Game/TurnBasedGame/Blueprints/Player/BP_PlayerActions.Grid` (`self.PlayerActions`)) "NewEnumerator3")
  ;[1 1 1] only get valid neigbors of the selected tile, e.g. no obstacles, flying only spots or edge of the map
  (bind _neighbors (`/Game/TurnBasedGame/Blueprints/Grid/BP_Pathfinding.GetValidTileNeighbors` (`/Game/TurnBasedGame/Blueprints/Grid/BP_Grid.GridPathfinding` (`/Game/TurnBasedGame/Blueprints/Player/BP_PlayerActions.Grid` (`self.PlayerActions`))) (`local.Index`) (`self.IncludeDiagonals`) (`|MakeArray` "NewEnumerator1" "NewEnumerator3" "NewEnumerator4" :!type "/Game/TurnBasedGame/Blueprints/Grid/Utilities/BPE_TypeTile Enum")))
  ;[1 1 1] add isNeighbor state to every neighboring tile to the selected tile.
  (for _array_element _neighbors
    (`/Game/TurnBasedGame/Blueprints/Grid/BP_Grid.AddStateToTile` (`/Game/TurnBasedGame/Blueprints/Player/BP_PlayerActions.Grid` (`self.PlayerActions`)) (break `/Game/TurnBasedGame/Blueprints/Grid/Utilities/BPS_DataPathfinding` _array_element) "NewEnumerator3")))

(fn `UserConstructionScript`
  (`parent.UserConstructionScript`))