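; Player action Blueprint for the turn-based grid game that computes the minimum pathfinding cost from every grid tile to the currently selected tile.
; On execute it clears the pathfinding's generated data and, if the selected tile is valid, loops over all grid tiles.
; Each tile is registered as discovered with zero start cost and its minimum cost to the selection, optionally counting diagonals.
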(fn `CalculateCostFromSelectedTileToAllOtherTiles`
  (bind _playeractions (`self.PlayerActions`))
  (bind _grid (`/Game/TurnBasedGame/Blueprints/Player/BP_PlayerActions.Grid` _playeractions))
  (bind _keys (`BlueprintMapLibrary.Map_Keys` (`/Game/TurnBasedGame/Blueprints/Grid/BP_Grid.GridTiles` _grid)))
  (for _array_element _keys
    (`/Game/TurnBasedGame/Blueprints/Grid/BP_Pathfinding.DiscoverTile` (`/Game/TurnBasedGame/Blueprints/Grid/BP_Grid.GridPathfinding` (`/Game/TurnBasedGame/Blueprints/Player/BP_PlayerActions.Grid` (`self.PlayerActions`))) (make `/Game/TurnBasedGame/Blueprints/Grid/Utilities/BPS_DataPathfinding` _array_element 1 0 (`/Game/TurnBasedGame/Blueprints/Grid/BP_Pathfinding.GetMinimumCostBetweenTwoTiles` (`/Game/TurnBasedGame/Blueprints/Grid/BP_Grid.GridPathfinding` _grid) _array_element (`/Game/TurnBasedGame/Blueprints/Player/BP_PlayerActions.SelectedTile` _playeractions) (`self.IncludeDiagonals`))))))

(fn `ExecuteAction`
  (params (Index :type "IntPoint Structure"))
  (bind _playeractions (`self.PlayerActions`))
  (`parent.ExecuteAction` Index)
  (`/Game/TurnBasedGame/Blueprints/Grid/BP_Pathfinding.ClearGeneratedData` (`/Game/TurnBasedGame/Blueprints/Grid/BP_Grid.GridPathfinding` (`/Game/TurnBasedGame/Blueprints/Player/BP_PlayerActions.Grid` (`self.PlayerActions`))))
  (if (`/Game/TurnBasedGame/Blueprints/Grid/BP_Grid.CheckIsIndexValid` (`/Game/TurnBasedGame/Blueprints/Player/BP_PlayerActions.Grid` _playeractions) (`/Game/TurnBasedGame/Blueprints/Player/BP_PlayerActions.SelectedTile` _playeractions))
    (`self.CalculateCostFromSelectedTileToAllOtherTiles`)))

(fn `UserConstructionScript`
  (`parent.UserConstructionScript`))