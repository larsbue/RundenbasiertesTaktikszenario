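; Grid action for the turn-based game that raises or lowers the height of the tile at a given index.
; ExecuteAction validates the index, reads that tile's data from the grid's GridTiles map and offsets its Z location by one GridTileSize.Z step, with the Increase flag choosing the direction.
; The edited data is written back through AddGridTile, keeping type, rotation, scale, states and unit unchanged.
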(fn `ExecuteAction`
  (params (Index :type "IntPoint Structure"))
  (locals (Data :type "/Game/TurnBasedGame/Blueprints/Grid/Utilities/BPS_DataTile Structure"))
  (bind (_gridtilesize_x _gridtilesize_y _gridtilesize_z) (`KismetMathLibrary.BreakVector` (`/Game/TurnBasedGame/Blueprints/Grid/BP_Grid.GridTileSize` (`/Game/TurnBasedGame/Blueprints/Player/BP_PlayerActions.Grid` (`self.PlayerActions`)))))
  (if (`/Game/TurnBasedGame/Blueprints/Grid/BP_Grid.IsIndexValid` (`/Game/TurnBasedGame/Blueprints/Player/BP_PlayerActions.Grid` (`self.PlayerActions`)) (`local.Index`))
    ;[1 1 1] find the data by fetching the index of the grid tiles array.
    (bind _output_get (set `local.Data` (`BlueprintMapLibrary.Map_Find` (`/Game/TurnBasedGame/Blueprints/Grid/BP_Grid.GridTiles` (`/Game/TurnBasedGame/Blueprints/Player/BP_PlayerActions.Grid` (`self.PlayerActions`))) (`local.Index`))))
    (`/Game/TurnBasedGame/Blueprints/Grid/BP_Grid.AddGridTile` (`/Game/TurnBasedGame/Blueprints/Player/BP_PlayerActions.Grid` (`self.PlayerActions`)) (make `/Game/TurnBasedGame/Blueprints/Grid/Utilities/BPS_DataTile` (break `/Game/TurnBasedGame/Blueprints/Grid/Utilities/BPS_DataTile` _output_get) (`.Type_6_5F1D582544258A461E8CED80E64FB436` (break `/Game/TurnBasedGame/Blueprints/Grid/Utilities/BPS_DataTile` _output_get)) (`KismetMathLibrary.MakeTransform` (+ (.location (`.Transform_8_4368262E41BF048BC408BDB4D4AEF3EB` (break `/Game/TurnBasedGame/Blueprints/Grid/Utilities/BPS_DataTile` _output_get))) (`KismetMathLibrary.MakeVector` 0.0 0.0 (* _gridtilesize_z (`KismetMathLibrary.SelectFloat` 1.0 -1.0 (`self.Increase`))))) (.rotation (`.Transform_8_4368262E41BF048BC408BDB4D4AEF3EB` (break `/Game/TurnBasedGame/Blueprints/Grid/Utilities/BPS_DataTile` _output_get))) (.scale (`.Transform_8_4368262E41BF048BC408BDB4D4AEF3EB` (break `/Game/TurnBasedGame/Blueprints/Grid/Utilities/BPS_DataTile` _output_get)))) (`.States_12_E157DEAE415E97B85AD1F69681B85DC8` (break `/Game/TurnBasedGame/Blueprints/Grid/Utilities/BPS_DataTile` _output_get)) (`.UnitOnTile_15_1E34864C4E787D0AB34915A28704B28C` (break `/Game/TurnBasedGame/Blueprints/Grid/Utilities/BPS_DataTile` _output_get))))))

(fn `UserConstructionScript`
  (`parent.UserConstructionScript`))