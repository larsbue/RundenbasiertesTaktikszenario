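; BP_Action_AddTile is a player action that adds a new tile to the grid at a given index in a turn-based game.
; It only acts when that index is not already a valid tile.
; It gets location, rotation and scale from the grid, traces against the ground channel for the placement location, then calls AddGridTile with that transform.
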(fn `ExecuteAction`
  (params (Index :type "IntPoint Structure"))
  ;[1 1 1] check if tile with index is NOT valid. already valid tiles cant be added.
  (if (not (`/Game/TurnBasedGame/Blueprints/Grid/BP_Grid.IsIndexValid` (`/Game/TurnBasedGame/Blueprints/Player/BP_PlayerActions.Grid` (`self.PlayerActions`)) (`local.Index`)))
    (bind (_tilelocation _tilerotation _tilescale) (`self.GetGridLocationRotationAndScale` (`local.Index`)))
    ;[1 1 1] tiles can only be added to terrain. this is checked by tracing for the ground channel. this linetrace is only blocked by assets marked as "ground".
    (bind _outlocation (`/Game/TurnBasedGame/Blueprints/Grid/BP_Grid.TraceForGround` (`/Game/TurnBasedGame/Blueprints/Player/BP_PlayerActions.Grid` (`self.PlayerActions`)) _tilelocation))
    (`/Game/TurnBasedGame/Blueprints/Grid/BP_Grid.AddGridTile` (`/Game/TurnBasedGame/Blueprints/Player/BP_PlayerActions.Grid` (`self.PlayerActions`)) (make `/Game/TurnBasedGame/Blueprints/Grid/Utilities/BPS_DataTile` (`local.Index`) "NewEnumerator1" (`KismetMathLibrary.MakeTransform` _outlocation _tilerotation _tilescale)))))

(fn `GetGridLocationRotationAndScale`
  (params (GridIndex :type "IntPoint Structure"))
  (returns (TileLocation :type "Vector Structure") (TileRotation :type "Rotator Structure") (TileScale :type "Vector Structure"))
  (bind _grid (`/Game/TurnBasedGame/Blueprints/Player/BP_PlayerActions.Grid` (`self.PlayerActions`)))
  (return (`/Game/TurnBasedGame/Blueprints/Grid/BP_Grid.GetTileLocationFromGridIndex` _grid GridIndex) (`/Game/TurnBasedGame/Blueprints/Grid/BP_Grid.GetTileRotationFromGridIndex` _grid GridIndex) (`/Game/TurnBasedGame/Blueprints/Grid/BP_Grid.GetTileScale` _grid)))

(fn `UserConstructionScript`
  (`parent.UserConstructionScript`))