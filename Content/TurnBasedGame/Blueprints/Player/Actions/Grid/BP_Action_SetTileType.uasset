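; BP_Action_SetTileType is a player grid action that changes the type of the tile at a given index.
; It validates the index on the PlayerActions grid and looks up that tile's data in GridTiles.
; It then re-adds the tile through AddGridTile with the action's TileType, carrying over its index, transform, states and unit on tile.
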(fn `ExecuteAction`
  (params (Index :type "IntPoint Structure"))
  (locals (Data :type "/Game/TurnBasedGame/Blueprints/Grid/Utilities/BPS_DataTile Structure"))
  (if (`/Game/TurnBasedGame/Blueprints/Grid/BP_Grid.CheckIsIndexValid` (`/Game/TurnBasedGame/Blueprints/Player/BP_PlayerActions.Grid` (`self.PlayerActions`)) (`local.Index`))
    (bind _output_get (set `local.Data` (`BlueprintMapLibrary.Map_Find` (`/Game/TurnBasedGame/Blueprints/Grid/BP_Grid.GridTiles` (`/Game/TurnBasedGame/Blueprints/Player/BP_PlayerActions.Grid` (`self.PlayerActions`))) (`local.Index`))))
    (`/Game/TurnBasedGame/Blueprints/Grid/BP_Grid.AddGridTile` (`/Game/TurnBasedGame/Blueprints/Player/BP_PlayerActions.Grid` (`self.PlayerActions`)) (make `/Game/TurnBasedGame/Blueprints/Grid/Utilities/BPS_DataTile` (break `/Game/TurnBasedGame/Blueprints/Grid/Utilities/BPS_DataTile` _output_get) (`self.TileType`) (`.Transform_8_4368262E41BF048BC408BDB4D4AEF3EB` (break `/Game/TurnBasedGame/Blueprints/Grid/Utilities/BPS_DataTile` _output_get)) (`.States_12_E157DEAE415E97B85AD1F69681B85DC8` (break `/Game/TurnBasedGame/Blueprints/Grid/Utilities/BPS_DataTile` _output_get)) (`.UnitOnTile_15_1E34864C4E787D0AB34915A28704B28C` (break `/Game/TurnBasedGame/Blueprints/Grid/Utilities/BPS_DataTile` _output_get))))))

(fn `UserConstructionScript`
  (`parent.UserConstructionScript`))