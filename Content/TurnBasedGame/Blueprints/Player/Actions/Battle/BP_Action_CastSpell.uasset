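; Player battle action for casting a spell from the selected tile at a target tile in the turn-based grid game.
; Setting a spell loads its cast and AoE data, then marks range tiles via grid tile states, refreshed on hover.
; When the hovered tile is in range, it marks the AoE pattern, or just that tile.
; Executing casts through Battle and deselects the spell button; EndPlay clears both highlights.
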(event `self.ReceiveEndPlay`
  (params (EndPlayReason :type "EEndPlayReason Enum" :default "Destroyed"))
  (bind _grid (`/Game/TurnBasedGame/Blueprints/Player/BP_PlayerActions.Grid` (`self.PlayerActions`)))
  (`parent.ReceiveEndPlay` EndPlayReason)
  ;[1 1 1] clear all leftover tile states after action is done.
  (`/Game/TurnBasedGame/Blueprints/Grid/BP_Grid.ClearStateFromTiles` _grid "NewEnumerator8")
  (`/Game/TurnBasedGame/Blueprints/Grid/BP_Grid.ClearStateFromTiles` _grid "NewEnumerator9"))

(fn `AddRangeStateToTilesInRange`
  (params (State :type "/Game/TurnBasedGame/Blueprints/Grid/Utilities/BPE_StateTile Enum" :default "NewEnumerator0") (Cast :type "/Game/TurnBasedGame/Blueprints/Battle/Spells/Utilities/BPS_SpellData_Cast Structure"))
  (bind _playeractions (`self.PlayerActions`))
  (bind _rangeindexes (`/Game/TurnBasedGame/Blueprints/Battle/BP_Battle.GetSpellRange` (`/Game/TurnBasedGame/Blueprints/Player/BP_PlayerActions.Battle` _playeractions) (`/Game/TurnBasedGame/Blueprints/Player/BP_PlayerActions.SelectedTile` _playeractions) Cast))
  (for _array_element _rangeindexes
    (`/Game/TurnBasedGame/Blueprints/Grid/BP_Grid.AddStateToTile` (`/Game/TurnBasedGame/Blueprints/Player/BP_PlayerActions.Grid` (`self.PlayerActions`)) _array_element State)))

(fn `ExecuteAction`
  (params (Index :type "IntPoint Structure"))
  (bind _w_battle (`/Game/TurnBasedGame/Blueprints/Player/BP_PlayerActions.W_Battle` (`self.PlayerActions`)))
  (`parent.ExecuteAction` Index)
  (`/Game/TurnBasedGame/Blueprints/Battle/BP_Battle.CastSpell` (`/Game/TurnBasedGame/Blueprints/Player/BP_PlayerActions.Battle` (`self.PlayerActions`)) (`self.Spell`) (`/Game/TurnBasedGame/Blueprints/Player/BP_PlayerActions.SelectedTile` (`self.PlayerActions`)) (`local.Index`))
  (`/Engine/EditorBlueprintResources/StandardMacros.IsValid` _w_battle
    (:`Is Valid`
      (`/Game/TurnBasedGame/Blueprints/Battle/Spells/Widgets/W_ButtonList_Spells.SetSelectedSpellFromIndex` (`/Game/TurnBasedGame/Blueprints/Battle/Widgets/W_Battle.ButtonList_Spells` _w_battle) -1))))

(fn `ExecuteHoveredAction`
  (params (Index :type "IntPoint Structure"))
  (`parent.ExecuteHoveredAction` Index)
  (`self.ShowSpellPattern`))

(fn `GetSpellRangeOfSpell`
  (bind _spelldata (`/Game/TurnBasedGame/Blueprints/Battle/Spells/Utilities/BFL_Spells.GetSpellDataFromSpell` (`self.Spell`)))
  (set `self.Cast` (`.Cast_9_85698F044021D8C8E332F89A44EF936C` (break `/Game/TurnBasedGame/Blueprints/Battle/Spells/Utilities/BPS_SpellData` _spelldata)))
  (set `self.CastAoe` (`.CastAoe_12_B98B359D49D9D94DEBDFC1ABA6AB6DB2` (break `/Game/TurnBasedGame/Blueprints/Battle/Spells/Utilities/BPS_SpellData` _spelldata)))
  (`self.ShowSpellPattern`))

(fn `SetSpell`
  (params (Spell :type "/Game/TurnBasedGame/Blueprints/Battle/Spells/Utilities/BPE_Spell Enum" :default "NewEnumerator0"))
  (bind _grid (`/Game/TurnBasedGame/Blueprints/Player/BP_PlayerActions.Grid` (`self.PlayerActions`)))
  (bind _output_get (set `self.Spell` Spell))
  (if (`|EnumInequality` _output_get "NewEnumerator0")
    (`self.GetSpellRangeOfSpell`)
    (else
      ;[1 1 1] clear tile states if no spell is selected.
      (`/Game/TurnBasedGame/Blueprints/Grid/BP_Grid.ClearStateFromTiles` _grid "NewEnumerator8")
      (`/Game/TurnBasedGame/Blueprints/Grid/BP_Grid.ClearStateFromTiles` _grid "NewEnumerator9"))))

(fn `ShowSpellPattern`
  (bind _playeractions (`self.PlayerActions`))
  (`|ExecutionSequence`
    (:`then_0`
      (`/Game/TurnBasedGame/Blueprints/Grid/BP_Grid.ClearStateFromTiles` (`/Game/TurnBasedGame/Blueprints/Player/BP_PlayerActions.Grid` (`self.PlayerActions`)) "NewEnumerator8")
      (bind _rangeindexes (`/Game/TurnBasedGame/Blueprints/Battle/BP_Battle.GetSpellRange` (`/Game/TurnBasedGame/Blueprints/Player/BP_PlayerActions.Battle` _playeractions) (`/Game/TurnBasedGame/Blueprints/Player/BP_PlayerActions.SelectedTile` _playeractions) (`self.Cast`)))
      (for _array_element _rangeindexes
        (`/Game/TurnBasedGame/Blueprints/Grid/BP_Grid.AddStateToTile` (`/Game/TurnBasedGame/Blueprints/Player/BP_PlayerActions.Grid` (`self.PlayerActions`)) _array_element "NewEnumerator8")))
    (:`then_1`
      (`self.ShowSpellPatternAoe`))))

(fn `ShowSpellPatternAoe`
  (`/Game/TurnBasedGame/Blueprints/Grid/BP_Grid.ClearStateFromTiles` (`/Game/TurnBasedGame/Blueprints/Player/BP_PlayerActions.Grid` (`self.PlayerActions`)) "NewEnumerator9")
  (if (`KismetArrayLibrary.Array_Contains` (`.IntPointArray_3_2057B2014BFE1BF278D315AC59D06B5C` (break `/Game/TurnBasedGame/Blueprints/Grid/Utilities/BPS_IntPointArray` (`BlueprintMapLibrary.Map_Find` (`/Game/TurnBasedGame/Blueprints/Grid/BP_Grid.TileStateToIndexes` (`/Game/TurnBasedGame/Blueprints/Player/BP_PlayerActions.Grid` (`self.PlayerActions`))) "NewEnumerator8"))) (`/Game/TurnBasedGame/Blueprints/Player/BP_PlayerActions.HoveredTile` (`self.PlayerActions`)))
    (if (`|EnumInequality` (`.Pattern_3_B6918C5140E88F74783679B58B5E549F` (break `/Game/TurnBasedGame/Blueprints/Battle/Spells/Utilities/BPS_SpellData_Cast` (`self.CastAoe`))) "NewEnumerator0")
      (`self.AddRangeStateToTilesInRange` "NewEnumerator9" (`self.CastAoe`))
      (else
        (`/Game/TurnBasedGame/Blueprints/Grid/BP_Grid.AddStateToTile` (`/Game/TurnBasedGame/Blueprints/Player/BP_PlayerActions.Grid` (`self.PlayerActions`)) (`/Game/TurnBasedGame/Blueprints/Player/BP_PlayerActions.HoveredTile` (`self.PlayerActions`)) "NewEnumerator9")))))

(fn `UserConstructionScript`
  (`parent.UserConstructionScript`))