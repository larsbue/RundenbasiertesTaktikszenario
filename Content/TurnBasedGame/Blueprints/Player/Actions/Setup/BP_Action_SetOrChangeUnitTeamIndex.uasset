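; Player setup action that sets or changes the team index of the unit standing on a selected grid tile.
; ExecuteAction looks up the tile by index in the grid's tile map and, if a valid unit is on it, passes that unit and the action's TeamIndex to the Battle's SetUnitTeamIndex.
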(fn `ExecuteAction`
  (params (Index :type "IntPoint Structure"))
  (bind ((`UnitOnTile_15_1E34864C4E787D0AB34915A28704B28C` _unitontile)) (break `/Game/TurnBasedGame/Blueprints/Grid/Utilities/BPS_DataTile` (`BlueprintMapLibrary.Map_Find` (`/Game/TurnBasedGame/Blueprints/Grid/BP_Grid.GridTiles` (`/Game/TurnBasedGame/Blueprints/Player/BP_PlayerActions.Grid` (`self.PlayerActions`))) (`local.Index`))))
  ;[1 1 1] set the team index of unit on tile if valid.
  (`/Engine/EditorBlueprintResources/StandardMacros.IsValid` _unitontile
    (:`Is Valid`
      (`/Game/TurnBasedGame/Blueprints/Battle/BP_Battle.SetUnitTeamIndex` (`/Game/TurnBasedGame/Blueprints/Player/BP_PlayerActions.Battle` (`self.PlayerActions`)) _unitontile (`self.TeamIndex`)))))

(fn `UserConstructionScript`
  (`parent.UserConstructionScript`))