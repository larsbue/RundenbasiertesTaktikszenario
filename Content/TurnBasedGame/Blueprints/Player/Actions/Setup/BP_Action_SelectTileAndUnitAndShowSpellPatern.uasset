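; Player action for the turn-based grid that highlights a spell's cast range and area-of-effect pattern as tile states.
; On execute, it clears old range states, marks tiles the CombatSystem returns for the selected tile, then refreshes the AoE.
; Hover also refreshes AoE, shown only while the hovered tile is in range.
; Patternless AoE marks the hovered tile; patterned AoE reuses the range helper, which originates at the selected tile.
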(fn `AddRangeStateToTilesInRange`
  (params (State :type "/Game/TurnBasedGame/Blueprints/Grid/Utilities/BPE_StateTile Enum" :default "NewEnumerator0") (Cast :type "/Game/TurnBasedGame/Blueprints/Combat/Spells/Utilities/BPS_SpellData_Cast Structure"))
  (bind _playeractions (`self.PlayerActions`))
  (bind _rangeindexes (`/Game/TurnBasedGame/Blueprints/Combat/BP_Combat.GetSpellRange` (`/Game/TurnBasedGame/Blueprints/Player/BP_PlayerActions.CombatSystem` _playeractions) (`/Game/TurnBasedGame/Blueprints/Player/BP_PlayerActions.SelectedTile` _playeractions) Cast))
  (for _array_element _rangeindexes
    (`/Game/TurnBasedGame/Blueprints/Grid/BP_Grid.AddStateToTile` (`/Game/TurnBasedGame/Blueprints/Player/BP_PlayerActions.Grid` (`self.PlayerActions`)) _array_element State)))

(fn `ExecuteAction`
  (params (Index :type "IntPoint Structure"))
  (`parent.ExecuteAction` Index)
  (`self.ShowSpellPattern`))

(fn `ExecuteHoveredAction`
  (params (Index :type "IntPoint Structure"))
  (`parent.ExecuteHoveredAction` Index)
  (`self.ShowSpellPatternAoe`))

(fn `ShowSpellPattern`
  (bind _playeractions (`self.PlayerActions`))
  (`|ExecutionSequence`
    (:`then_0`
      ;[1 1 1] first, clear all isSpellRange-states from tiles.
      (`/Game/TurnBasedGame/Blueprints/Grid/BP_Grid.ClearStateFromTiles` (`/Game/TurnBasedGame/Blueprints/Player/BP_PlayerActions.Grid` (`self.PlayerActions`)) "NewEnumerator8")
      ;[1 1 1] then, if the selected tile is valid, process all tiles in spell range and iterate over them to set the correct tile state.
      (if (`/Game/TurnBasedGame/Blueprints/Grid/BP_Grid.IsIndexValid` (`/Game/TurnBasedGame/Blueprints/Player/BP_PlayerActions.Grid` _playeractions) (`/Game/TurnBasedGame/Blueprints/Player/BP_PlayerActions.SelectedTile` _playeractions))
        (`self.AddRangeStateToTilesInRange` "NewEnumerator8" (`self.SpellDataCast`))))
    (:`then_1`
      ;[1 1 1] additionally, process aoe pattern.
      (`self.ShowSpellPatternAoe`))))

(fn `ShowSpellPatternAoe`
  (`/Game/TurnBasedGame/Blueprints/Grid/BP_Grid.ClearStateFromTiles` (`/Game/TurnBasedGame/Blueprints/Player/BP_PlayerActions.Grid` (`self.PlayerActions`)) "NewEnumerator9")
  (if (`KismetArrayLibrary.Array_Contains` (`.IntPointArray_3_2057B2014BFE1BF278D315AC59D06B5C` (break `/Game/TurnBasedGame/Blueprints/Grid/Utilities/BPS_IntPointArray` (`BlueprintMapLibrary.Map_Find` (`/Game/TurnBasedGame/Blueprints/Grid/BP_Grid.TileStateToIndexes` (`/Game/TurnBasedGame/Blueprints/Player/BP_PlayerActions.Grid` (`self.PlayerActions`))) "NewEnumerator8"))) (`/Game/TurnBasedGame/Blueprints/Player/BP_PlayerActions.HoveredTile` (`self.PlayerActions`)))
    ;[1 1 1] only display area of effect spell range if spell has area of effect pattern.
    (if (`|EnumInequality` (`.Pattern_3_B6918C5140E88F74783679B58B5E549F` (break `/Game/TurnBasedGame/Blueprints/Combat/Spells/Utilities/BPS_SpellData_Cast` (`self.SpellDataCastAoe`))) "NewEnumerator0")
      (`self.AddRangeStateToTilesInRange` "NewEnumerator9" (`self.SpellDataCastAoe`))
      (else
        (`/Game/TurnBasedGame/Blueprints/Grid/BP_Grid.AddStateToTile` (`/Game/TurnBasedGame/Blueprints/Player/BP_PlayerActions.Grid` (`self.PlayerActions`)) (`/Game/TurnBasedGame/Blueprints/Player/BP_PlayerActions.HoveredTile` (`self.PlayerActions`)) "NewEnumerator9")))))

(fn `UserConstructionScript`
  (`parent.UserConstructionScript`))