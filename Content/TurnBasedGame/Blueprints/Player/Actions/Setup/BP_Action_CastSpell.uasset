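; A player action blueprint that casts the configured spell on the clicked tile as a debug tool.
; ExecuteAction calls CastSpell on the battle from the selected tile to the given tile index.
; If a unit is selected, it then resets that unit's action points, so the spell costs nothing to test.
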(event `self.ReceiveBeginPlay`
  (`parent.ReceiveBeginPlay`))

(event `self.ReceiveEndPlay`
  (params (EndPlayReason :type "EEndPlayReason Enum" :default "Destroyed"))
  (`parent.ReceiveEndPlay` EndPlayReason))

(fn `ExecuteAction`
  (params (Index :type "IntPoint Structure"))
  (bind _selectedunit (`/Game/TurnBasedGame/Blueprints/Player/BP_PlayerActions.SelectedUnit` (`self.PlayerActions`)))
  ;[1 1 1] debug function to cast selected spell and reset ap if unit is selected and valid.
  (`/Game/TurnBasedGame/Blueprints/Battle/BP_Battle.CastSpell` (`/Game/TurnBasedGame/Blueprints/Player/BP_PlayerActions.Battle` (`self.PlayerActions`)) (`self.Spell`) (`/Game/TurnBasedGame/Blueprints/Player/BP_PlayerActions.SelectedTile` (`self.PlayerActions`)) (`local.Index`))
  (`/Engine/EditorBlueprintResources/StandardMacros.IsValid` _selectedunit
    (:`Is Valid`
      (`/Game/TurnBasedGame/Blueprints/Unit/BP_Unit.ResetAp` _selectedunit))))

(fn `UserConstructionScript`
  (`parent.UserConstructionScript`))