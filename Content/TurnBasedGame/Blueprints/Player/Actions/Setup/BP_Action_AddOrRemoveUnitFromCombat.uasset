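; A player action for combat setup that adds or removes a unit on a given grid tile.
; When adding, it checks that the tile type is valid for the unit type, destroys any existing occupant, then spawns a BP_Unit and registers it with the CombatSystem using team and AI settings.
; When removing, it reuses the same removal branch to take the tile's unit out of combat and destroy it.
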(fn `ExecuteAction`
  (params (Index :type "IntPoint Structure"))
  (bind ((`UnitOnTile_15_1E34864C4E787D0AB34915A28704B28C` _unitontile)) (break `/Game/TurnBasedGame/Blueprints/Grid/Utilities/BPS_DataTile` (`BlueprintMapLibrary.Map_Find` (`/Game/TurnBasedGame/Blueprints/Grid/BP_Grid.GridTiles` (`/Game/TurnBasedGame/Blueprints/Player/BP_PlayerActions.Grid` (`self.PlayerActions`))) (`local.Index`))))
  (if (`self.IsAddingUnit`)
    ;[1 1 1] check if unit is placebale on selected tile by type
    (bind _unitdata (`/Game/TurnBasedGame/Blueprints/Units/Utilities/BFL_Units.GetDefaultUnitDataFromUnitType` (`self.UnitType`)))
    (if (`KismetArrayLibrary.Array_Contains` (break `/Game/TurnBasedGame/Blueprints/Units/Utilities/BPS_Unit_Stats` (`.Stats_8_59677AC742C58E50C0B0B8BFC3DDDE60` (break `/Game/TurnBasedGame/Blueprints/Units/Utilities/BPS_Unit` _unitdata))) (`.Type_6_5F1D582544258A461E8CED80E64FB436` (break `/Game/TurnBasedGame/Blueprints/Grid/Utilities/BPS_DataTile` (`BlueprintMapLibrary.Map_Find` (`/Game/TurnBasedGame/Blueprints/Grid/BP_Grid.GridTiles` (`/Game/TurnBasedGame/Blueprints/Player/BP_PlayerActions.Grid` (`self.PlayerActions`))) (`local.Index`)))))
      (`|ExecutionSequence`
        (:`then_0`
          ;[1 1 1] if unit is valid and action is not adding unit, delete the unit by destroying its actor
          (`/Engine/EditorBlueprintResources/StandardMacros.IsValid` _unitontile :!label _label
            (:`Is Valid`
              (`/Game/TurnBasedGame/Blueprints/Combat/BP_Combat.RemoveUnitFromCombat` (`/Game/TurnBasedGame/Blueprints/Player/BP_PlayerActions.CombatSystem` (`self.PlayerActions`)) _unitontile true))))
        (:`then_1`
          ;[1 1 1] spawns unit actor in world with selected unit type, team index and selected tile. also select if unit shall be controlled by ai
          (bind _returnvalue (`|SpawnActorFromClass` "/Game/TurnBasedGame/Blueprints/Units/BP_Unit.BP_Unit_C" (`KismetMathLibrary.MakeTransform` (0.0 0.0 0.0)) "AlwaysSpawn" "MultiplyWithRoot" null (`self.UnitType`) null))
          (`/Game/TurnBasedGame/Blueprints/Combat/BP_Combat.AddUnitToCombat` (`/Game/TurnBasedGame/Blueprints/Player/BP_PlayerActions.CombatSystem` (`self.PlayerActions`)) _returnvalue (`local.Index`) (`self.TeamIndex`) (`self.UseAI`)))))
    (else
      (goto _label))))

(fn `UserConstructionScript`
  (`parent.UserConstructionScript`))