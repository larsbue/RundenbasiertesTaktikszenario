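; Base turn AI for a battle unit in a grid-based, turn-based game.
; An event-chained state flow repeatedly picks a spell, moves and casts, then moves to an end position and passes the turn.
; Spell choice brute-forces castable spells, reachable origins and targets, scoring distance and HP impact over AP cost.
; End position follows the unit's approach/retreat logic, using async pathfinding; in-battle checks halt the flow between steps.
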(event `self.ReceiveBeginPlay`
  (add `/Game/TurnBasedGame/Blueprints/Unit/BP_Unit.OnUnitIsInBattleChanged` (`self.Unit`) (delegate `OnUnitActiveinBattleChanged`)))

(event `OnUnitActiveinBattleChanged`
  (params (Unit :type "/Game/TurnBasedGame/Blueprints/Unit/BP_Unit Object Reference"))
  ;[1 1 1] check if unit is still in battle. if not, set ai state to endturn and therefore end the flow.
  (if (`/Game/TurnBasedGame/Blueprints/Unit/BP_Unit.IsInBattle` Unit)
    _
    (elif (`|EnumInequality` (`self.AIState`) "NewEnumerator7")
      (set `self.AIState` "NewEnumerator7")
      (`self.OnAIStateChanged` self))))

(event `CastSelectedSpell_Done`
  ;[1 1 1] coming from State 4: start over to check if more spells can be cast.
  ;[1 1 1] State 2: initiate the flow by choosing a spell to cast.
  (`self.DelayBetweenStates` "NewEnumerator2" :!label _label
    (:`Completed`
      (`self.ChooseSpell`))))

(event `InitiateAIFlow`
  ;[1 1 1] State 2: initiate the flow by choosing a spell to cast.
  (`self.DelayBetweenStates` "NewEnumerator1"
    (:`Completed`
      (goto _label))))

(event `ChooseSpell_Done`
  ;[1 1 1] State 3: check if any spell was chosen by checking if it is valid. if its valid, move to the calculated best casting position.
  (if (`.IsSpellValid_1_FC3B9EE14061073AEBE78B909C85060D` (break `/Game/TurnBasedGame/Blueprints/AI/S_UnitAISpellCastData` (`self.AISpellCast`)))
    (`self.DelayBetweenStates` "NewEnumerator3"
      (:`Completed`
        (`self.MoveToSpellPosition`)))
    (else
      ;[1 1 1] State 5: if its not valid, calculate the position to end the round.
      (`self.DelayBetweenStates` "NewEnumerator5"
        (:`Completed`
          (`self.DetermineEndPosition`))))))

(event `MoveToSpellPosition_Done`
  ;[1 1 1] State 4: cast the spell.
  (`self.DelayBetweenStates` "NewEnumerator4"
    (:`Completed`
      (`self.CastSelectedSpell`))))

(event `DetermineEndPosition_Done`
  (params (Path :type "Array of IntPoint Structure"))
  ;[1 1 1] State 6: move to the calculated end turn position
  (`self.DelayBetweenStates` "NewEnumerator6"
    (:`Completed`
      (`self.MoveToEndPosition` Path))))

(event `MoveToEndPosition_Done`
  ;[1 1 1] State 7: end the ai flow after reaching the end position.
  (`self.DelayBetweenStates` "NewEnumerator7"
    (:`Completed`
      (`self.AIEndTurn`))))

(event `DetermineEndPosition`
  ;[1 1 1] return empty array (no path), if no more move points left.
  (if (> (`.MP_Current_9_342C6130430EBE8DE80D35B13735B31E` (break `/Game/TurnBasedGame/Blueprints/Unit/Utilities/BPS_Unit_Stats` (`.Stats_8_59677AC742C58E50C0B0B8BFC3DDDE60` (break `/Game/TurnBasedGame/Blueprints/Unit/Utilities/BPS_Unit` (`/Game/TurnBasedGame/Blueprints/Unit/BP_Unit.UnitData` (`self.Unit`)))))) 0)
    ;[1 1 1] if unit has move points left, calculate all reachable tiles.
    (add `/Game/TurnBasedGame/Blueprints/Grid/BP_Pathfinding.OnPathfindingCompleted` (`self.AIGetPathfinding`) (delegate `OnCompleted_EndTurnPathWithReachableTiles`))
    (`self.AIGetPathWithReachableTiles`)
    (else
      (`self.DetermineEndPosition_Done` (`|MakeArray`)))))

(event `OnCompleted_EndTurnPathWithReachableTiles`
  (params (Path :type "Array of IntPoint Structure (by ref)"))
  ;[1 1 1] after the reachable tiles are calculated, find the best tile to move the unit to by using the units ai move logic.
  (remove `/Game/TurnBasedGame/Blueprints/Grid/BP_Pathfinding.OnPathfindingCompleted` (`self.AIGetPathfinding`) (delegate `OnCompleted_EndTurnPathWithReachableTiles`))
  (`self.StopIfNotInBattle`)
  (bind _bestindex (`self.AIFindBestIndexInReachableTiles` Path))
  ;[1 1 1] calculate a path to the calculated best index.
  (add `/Game/TurnBasedGame/Blueprints/Grid/BP_Pathfinding.OnPathfindingCompleted` (`self.AIGetPathfinding`) (delegate `OnComplete_EndTurnPath`))
  (`self.AIGetPathWithoutReachableTiles` _bestindex))

(event `OnComplete_EndTurnPath`
  (params (Path :type "Array of IntPoint Structure (by ref)"))
  ;[1 1 1] after the path is calculated, continue to the next ai flow state.
  (remove `/Game/TurnBasedGame/Blueprints/Grid/BP_Pathfinding.OnPathfindingCompleted` (`self.AIGetPathfinding`) (delegate `OnComplete_EndTurnPath`))
  (`self.StopIfNotInBattle`)
  (`self.DetermineEndPosition_Done` Path))

(event `MoveToEndPosition`
  (params (Path :type "Array of IntPoint Structure"))
  ;[1 1 1] if the best possible position is the one the unit is standing on (path length = 0), dont move.
  (if (> (`KismetArrayLibrary.Array_Length` Path) 0)
    ;[1 1 1] otherwise, move the unit analogous to the moving to spell casting position.
    (add `/Game/TurnBasedGame/Blueprints/Unit/BP_Unit.OnUnitFinishedWalking` (`self.Unit`) (delegate `OnCompleted_EndTurnUnitWalking`))
    (`/Game/TurnBasedGame/Blueprints/Battle/BP_Battle.MoveUnit` (`self.Battle`) (`self.Unit`) Path)
    (else
      (`self.MoveToEndPosition_Done`))))

(event `OnCompleted_EndTurnUnitWalking`
  (params (Unit :type "/Game/TurnBasedGame/Blueprints/Unit/BP_Unit Object Reference"))
  ;[1 1 1] wait for the move operation to end before going to the next ai flow state.
  (remove `/Game/TurnBasedGame/Blueprints/Unit/BP_Unit.OnUnitFinishedWalking` Unit (delegate `OnCompleted_EndTurnUnitWalking`))
  (`self.StopIfNotInBattle`)
  (`self.MoveToEndPosition_Done`))

(event `ChooseSpell`
  ;[1 1 1] first, clear the spell list.
  (set `self.AISpellCast` (struct))
  ;[1 1 1] get an array with all reachable tiles to check over.
  (add `/Game/TurnBasedGame/Blueprints/Grid/BP_Pathfinding.OnPathfindingCompleted` (`self.AIGetPathfinding`) (delegate `OnCompleted_SpellPathWithReachableTiles`))
  (`self.AIGetPathWithReachableTiles`))

(event `OnCompleted_SpellPathWithReachableTiles`
  (params (Path :type "Array of IntPoint Structure (by ref)"))
  ;[1 1 1] after the path is calculated, unbind from event. then choose the best spell to cast by checking all tiles in the path. after done, continue ai flow.
  (remove `/Game/TurnBasedGame/Blueprints/Grid/BP_Pathfinding.OnPathfindingCompleted` (`self.AIGetPathfinding`) (delegate `OnCompleted_SpellPathWithReachableTiles`))
  (`self.StopIfNotInBattle`)
  (`self.AIChooseBestSpellToCast` Path)
  (`self.ChooseSpell_Done`))

(event `MoveToSpellPosition`
  (bind ((`IsSpellValid_1_FC3B9EE14061073AEBE78B909C85060D` _isspellvalid) (`OriginIndex_9_68DA5BF241FEF5D5270F48879C43AE49` _originindex)) (break `/Game/TurnBasedGame/Blueprints/AI/S_UnitAISpellCastData` (`self.AISpellCast`)))
  ;[1 1 1] to move to the spell casting position, first check if the spell is valid AND the unit is not on the spell casting position yet. otherwise, just cast the spell from this position and dont move.
  (if (and (!= (`/Game/TurnBasedGame/Blueprints/Unit/BP_Unit.Index` (`self.Unit`)) _originindex) _isspellvalid)
    ;[1 1 1] calculate the actual path to the spell casting position.
    (add `/Game/TurnBasedGame/Blueprints/Grid/BP_Pathfinding.OnPathfindingCompleted` (`self.AIGetPathfinding`) (delegate `OnCompleted_SpellPath`))
    (`self.AIGetPathWithoutReachableTiles` (`.OriginIndex_9_68DA5BF241FEF5D5270F48879C43AE49` (break `/Game/TurnBasedGame/Blueprints/AI/S_UnitAISpellCastData` (`self.AISpellCast`))))
    (else
      (`self.MoveToSpellPosition_Done`))))

(event `OnCompleted_SpellPath`
  (params (Path :type "Array of IntPoint Structure (by ref)"))
  ;[1 1 1] after calculating the path, move to the end casting position using the calculated path.
  (remove `/Game/TurnBasedGame/Blueprints/Grid/BP_Pathfinding.OnPathfindingCompleted` (`self.AIGetPathfinding`) (delegate `OnCompleted_SpellPath`))
  (`self.StopIfNotInBattle`)
  (add `/Game/TurnBasedGame/Blueprints/Unit/BP_Unit.OnUnitFinishedWalking` (`self.Unit`) (delegate `OnCompleted_SpellUnitWalking`))
  (`/Game/TurnBasedGame/Blueprints/Battle/BP_Battle.MoveUnit` (`self.Battle`) (`self.Unit`) Path))

(event `OnCompleted_SpellUnitWalking`
  (params (Unit :type "/Game/TurnBasedGame/Blueprints/Unit/BP_Unit Object Reference"))
  ;[1 1 1] wait for the unit movement to finish before going to the next ai flow state.
  (remove `/Game/TurnBasedGame/Blueprints/Unit/BP_Unit.OnUnitFinishedWalking` Unit (delegate `OnCompleted_SpellUnitWalking`))
  (`self.StopIfNotInBattle`)
  (`self.MoveToSpellPosition_Done`))

(event `CastSelectedSpell`
  (bind ((`Spell_7_616A2B6D4F75A9B154D92CA70508ACB2` _spell) (`OriginIndex_9_68DA5BF241FEF5D5270F48879C43AE49` _originindex) (`TargetIndex_11_8B0E40804A75E9415E36888659DC095F` _targetindex)) (break `/Game/TurnBasedGame/Blueprints/AI/S_UnitAISpellCastData` (`self.AISpellCast`)))
  ;[1 1 1] check if spell is valid (as usual).
  (if (`.IsSpellValid_1_FC3B9EE14061073AEBE78B909C85060D` (break `/Game/TurnBasedGame/Blueprints/AI/S_UnitAISpellCastData` (`self.AISpellCast`)))
    ;[1 1 1] cast the calculated spell and wait for 0.5 seconds before going to the next state to let the animation play.
    (`/Game/TurnBasedGame/Blueprints/Battle/BP_Battle.CastSpell` (`self.Battle`) _spell _originindex _targetindex)
    (`KismetSystemLibrary.Delay` 0.5)
    (`self.StopIfNotInBattle`)
    (`self.CastSelectedSpell_Done`)
    (else
      (`self.CastSelectedSpell_Done`))))

(fn `AIBattleEnded`)

(fn `AIBattleStarted`)

(fn `AIBeginTurn`
  (`self.InitiateAIFlow`))

(fn `AICalculateApCost`
  (params (Spell :type "/Game/TurnBasedGame/Blueprints/Battle/Spells/Utilities/BPS_SpellData Structure"))
  (returns (ReturnValue :type "Float (double-precision)"))
  (return (* (`.ActionPointsCost_2_B2DF245A493C6B748782FCAFA215B290` (break `/Game/TurnBasedGame/Blueprints/Battle/Spells/Utilities/BPS_SpellData_Requirements` (`.Requirements_18_4281FB654CB40E08FCC5939ED071E8A6` (break `/Game/TurnBasedGame/Blueprints/Battle/Spells/Utilities/BPS_SpellData` Spell)))) (`self.HpValue`))))

(fn `AICalculateHpScore`
  (params (Spell :type "/Game/TurnBasedGame/Blueprints/Battle/Spells/Utilities/BPS_SpellData Structure") (AttackedUnit :type "/Game/TurnBasedGame/Blueprints/Unit/BP_Unit Object Reference") (IsAlly :type Boolean))
  (returns (Score :type "Float (double-precision)"))
  (bind _minmaxmodifier_hp (break `/Game/TurnBasedGame/Blueprints/Battle/Spells/Utilities/BPS_SpellData_Stats` (`.Stats_15_29A51BF842020762CC2E1FB71554CF3D` (break `/Game/TurnBasedGame/Blueprints/Battle/Spells/Utilities/BPS_SpellData` (`local.Spell`)))))
  (bind (_x _y) (break `IntPoint` _minmaxmodifier_hp))
  (bind ((`HP_Current_14_DF3407B84715BA0A38CA43B0D88C8ED4` _hp_current) (`HP_Max_15_6E7147AD427713A02E1E65ABFF535596` _hp_max)) (break `/Game/TurnBasedGame/Blueprints/Unit/Utilities/BPS_Unit_Stats` (`.Stats_8_59677AC742C58E50C0B0B8BFC3DDDE60` (break `/Game/TurnBasedGame/Blueprints/Unit/Utilities/BPS_Unit` (`/Game/TurnBasedGame/Blueprints/Unit/BP_Unit.UnitData` (`local.AttackedUnit`))))))
  (bind _returnvalue (- _hp_max _hp_current))
  (return (`self.AIStatScoreHandler` (select `bool` (> _x 0) :`false` _minmaxmodifier_hp :`true` (make `IntPoint` (`KismetMathLibrary.Min` _x _returnvalue) (`KismetMathLibrary.Min` _y _returnvalue))) (`local.IsAlly`))))

(fn `AICalculateKillingBlowScore`
  (params (Spell :type "/Game/TurnBasedGame/Blueprints/Battle/Spells/Utilities/BPS_SpellData Structure") (AttackedUnit :type "/Game/TurnBasedGame/Blueprints/Unit/BP_Unit Object Reference") (IsAlly :type Boolean))
  (returns (KillingBlowScore :type "Float (double-precision)"))
  (bind (_x _y) (break `IntPoint` (`.MinMaxModifier_Hp_2_337387544FC677D17537229603DB65D4` (break `/Game/TurnBasedGame/Blueprints/Battle/Spells/Utilities/BPS_SpellData_Stats` (`.Stats_15_29A51BF842020762CC2E1FB71554CF3D` (break `/Game/TurnBasedGame/Blueprints/Battle/Spells/Utilities/BPS_SpellData` (`local.Spell`)))))))
  (bind _returnvalue (`KismetMathLibrary.Conv_IntToDouble` (`KismetMathLibrary.Abs_Int` _x)))
  ;[1 1 1] if the spell is healing (modifier > 0), it wont kill so the killing blow score is always 0.
  (if (< (`.X` (break `IntPoint` (`.MinMaxModifier_Hp_2_337387544FC677D17537229603DB65D4` (break `/Game/TurnBasedGame/Blueprints/Battle/Spells/Utilities/BPS_SpellData_Stats` (`.Stats_15_29A51BF842020762CC2E1FB71554CF3D` (break `/Game/TurnBasedGame/Blueprints/Battle/Spells/Utilities/BPS_SpellData` (`local.Spell`))))))) 0)
    (return (* (`self.KillValue`) (`KismetMathLibrary.FClamp` (- 1.0 (/ (- (`KismetMathLibrary.Conv_IntToDouble` (`.HP_Current_14_DF3407B84715BA0A38CA43B0D88C8ED4` (break `/Game/TurnBasedGame/Blueprints/Unit/Utilities/BPS_Unit_Stats` (`.Stats_8_59677AC742C58E50C0B0B8BFC3DDDE60` (break `/Game/TurnBasedGame/Blueprints/Unit/Utilities/BPS_Unit` (`/Game/TurnBasedGame/Blueprints/Unit/BP_Unit.UnitData` (`local.AttackedUnit`))))))) _returnvalue) (- (+ (`KismetMathLibrary.Conv_IntToDouble` (`KismetMathLibrary.Abs_Int` _y)) 1.0) _returnvalue)))) (`KismetMathLibrary.SelectFloat` -1.0 1.0 (`local.IsAlly`))))
    (else
      (return 0.0))))

(fn `AIChooseBestSpellToCast`
  (params (ReachableTiles :type "Array of IntPoint Structure"))
  (bind _spells (`self.AIGetCastableSpells`))
  (bind _array_element (`/Game/TurnBasedGame/Blueprints/Utilities/StandardMacros.ManualForEachLoop` _spells :!label _label)
    (:`LoopBody`
      (bind _array_element_2 (`/Game/TurnBasedGame/Blueprints/Utilities/StandardMacros.ManualForEachLoop` ReachableTiles :!label _label_2)
        (:`LoopBody`
          (bind _rangeindexes (`/Game/TurnBasedGame/Blueprints/Battle/BP_Battle.GetSpellRange` (`self.Battle`) _array_element_2 (`.Cast_9_85698F044021D8C8E332F89A44EF936C` (break `/Game/TurnBasedGame/Blueprints/Battle/Spells/Utilities/BPS_SpellData` _array_element))))
          (bind _array_element_3 (`/Game/TurnBasedGame/Blueprints/Utilities/StandardMacros.ManualForEachLoop` _rangeindexes :!label _label_3)
            (:`LoopBody`
              (`self.AISpellCastHandler` _array_element_3 _array_element_2 _array_element)
              (goto _label_3 :!via `NextLoop`))
            (:`Completed`
              (goto _label_2 :!via `NextLoop`))))
        (:`Completed`
          (goto _label :!via `NextLoop`))))
    (:`Completed`
      (return))))

(fn `AIEndTurn`
  (`/Game/TurnBasedGame/Blueprints/Battle/BP_Battle.SwitchToNextUnit` (`self.Battle`)))

(fn `AIFindBestIndexInReachableTiles`
  (params (Reachables :type "Array of IntPoint Structure (by ref)"))
  (returns (BestIndex :type "IntPoint Structure"))
  (locals (Targets :type "Array of IntPoint Structure"))
  (bind _movelogic (`self.AIGetUnitMoveLogic`))
  ;[1 1 1] switch between different ai behaviour. this is the basic behaviour. to implement different logics for different unit types, override this class in the corresponding child class
  (`|ExecutionSequence`
    (:`then_0`
      (switch `/Game/TurnBasedGame/Blueprints/AI/E_AIMoveLogic` _movelogic
        (:`NewEnumerator0`
          (bind _units (`self.AIGetEnemyUnits` (`|MakeArray`) :!label _label))
          (bind _keys (`BlueprintMapLibrary.Map_Keys` _units))
          (set `local.Targets` _keys))
        (:`NewEnumerator1`
          (bind _units_2 (`self.AIGetAllyUnits` false :!label _label_2))
          (bind _keys_2 (`BlueprintMapLibrary.Map_Keys` _units_2))
          (bind _output_get (set `local.Targets` _keys_2))
          ;[1 1 1] incase there are no allies, move away from enemy units
          (if (== (`KismetArrayLibrary.Array_Length` _output_get) 0)
            (goto _label)))
        (:`NewEnumerator2`
          (goto _label))
        (:`NewEnumerator3`
          (goto _label_2))))
    (:`then_1`
      (switch `/Game/TurnBasedGame/Blueprints/AI/E_AIMoveLogic` _movelogic
        (:`NewEnumerator0`
          _)
        (:`NewEnumerator1`
          _)
        (:`NewEnumerator2`
          (bind _index (`self.AIFindFarthestIndex` (`local.Reachables`) (`local.Targets`) :!label _label_3))
          (return _index))
        (:`NewEnumerator3`
          (goto _label_3)))
      (bind _index_2 (`self.AIFindNearestIndex` (`local.Reachables`) (`local.Targets`)))
      (return _index_2))))

(fn `AIFindFarthestIndex`
  (params (ReachableTiles :type "Array of IntPoint Structure") (AvoidIndexes :type "Array of IntPoint Structure"))
  (returns (Index :type "IntPoint Structure"))
  (locals (ReturnIndex :type "IntPoint Structure") (LargestDistance :type Integer) (ReachableTile :type "IntPoint Structure") (TempLargestDistance :type Integer) (TileToAvoid :type "IntPoint Structure"))
  ;[1 1 1] find the farthest index in reachable tiles from current point
  ;[1 1 1] first, set biggest distance to unusual high value for later comparison
  (set `local.LargestDistance` -99999999)
  ;[1 1 1] iterate over all reachable tiles
  (for _array_element ReachableTiles
    (set `local.ReachableTile` _array_element)
    (set `local.TempLargestDistance` 99999999)
    ;[1 1 1] for each reachable tile iterate over all tiles to avoid (tiles with enemies)
    (for _array_element_2 (`local.AvoidIndexes`)
      (set `local.TileToAvoid` _array_element_2)
      ;[1 1 1] for every tile to avoid set temp largest distance to value with smallest gap between min cost of reachable tile and tile to avoid or the previous temp largest distance.
      (set `local.TempLargestDistance` (`KismetMathLibrary.Min` (`local.TempLargestDistance`) (`/Game/TurnBasedGame/Blueprints/Grid/BP_Pathfinding.GetMinimumCostBetweenTwoTiles` (`/Game/TurnBasedGame/Blueprints/Grid/BP_Grid.GridPathfinding_AI` (`/Game/TurnBasedGame/Blueprints/Battle/BP_Battle.Grid` (`self.Battle`))) (`local.ReachableTile`) (`local.TileToAvoid`) false))))
    ;[1 1 1] if temp largest distance is greater then the largest distance, set the value accordingly for later comparison
    (if (> (`local.TempLargestDistance`) (`local.LargestDistance`))
      (set `local.ReturnIndex` (`local.ReachableTile`))
      (set `local.LargestDistance` (`local.TempLargestDistance`))))
  (return (`local.ReturnIndex`)))

(fn `AIFindNearestIndex`
  (params (ReachableTiles :type "Array of IntPoint Structure") (PossibleTargets :type "Array of IntPoint Structure"))
  (returns (Index :type "IntPoint Structure"))
  (locals (SmallestDistance :type Integer) (ReachableTile :type "IntPoint Structure") (ReturnIndex :type "IntPoint Structure") (Target :type "IntPoint Structure") (TempSmallestDistance :type Integer :default 0))
  ;[1 1 1] finds the closest index to all possible targets in all reachable tiles
  ;[1 1 1] first, set distance to an unusual high value for later comparison
  (set `local.SmallestDistance` 99999999)
  ;[1 1 1] iterate over all reachable tiles and the possible targets.
  (for _array_element ReachableTiles
    (set `local.ReachableTile` _array_element)
    (for _array_element_2 (`local.PossibleTargets`)
      (set `local.Target` _array_element_2)
      ;[1 1 1] for every possible target, set the new smallest distance to the cost between the currently selected reachable tile and currently selected target and compare it to the smallest distance.
      (if (!= (`local.ReachableTile`) (`/Game/TurnBasedGame/Blueprints/Unit/BP_Unit.Index` (`self.Unit`)))
        (set `local.TempSmallestDistance` (`/Game/TurnBasedGame/Blueprints/Grid/BP_Pathfinding.GetMinimumCostBetweenTwoTiles` (`/Game/TurnBasedGame/Blueprints/Grid/BP_Grid.GridPathfinding_AI` (`/Game/TurnBasedGame/Blueprints/Battle/BP_Battle.Grid` (`self.Battle`))) (`local.ReachableTile`) (`local.Target`) (`.CanMoveDiagonal_4_93F482A44F4F1FD66CC945895CDB6EDC` (break `/Game/TurnBasedGame/Blueprints/Unit/Utilities/BPS_Unit_Stats` (`.Stats_8_59677AC742C58E50C0B0B8BFC3DDDE60` (break `/Game/TurnBasedGame/Blueprints/Unit/Utilities/BPS_Unit` (`/Game/TurnBasedGame/Blueprints/Unit/BP_Unit.UnitData` (`self.Unit`))))))))
        ;[1 1 1] set the smallest distance to temp smallest distance if it is lower.
        (if (< (`local.TempSmallestDistance`) (`local.SmallestDistance`))
          (set `local.ReturnIndex` (`local.ReachableTile`))
          (set `local.SmallestDistance` (`local.TempSmallestDistance`))))))
  (return (`local.ReturnIndex`)))

(fn `AIGetAllyUnits`
  (params (IsSelfIncluded :type Boolean))
  (returns (Units :type "Map of IntPoint Structure to /Game/TurnBasedGame/Blueprints/Unit/BP_Unit Object Reference"))
  (locals (ReturnUnits :type "Map of IntPoint Structure to /Game/TurnBasedGame/Blueprints/Unit/BP_Unit Object Reference") (Unit_Temp :type "/Game/TurnBasedGame/Blueprints/Unit/BP_Unit Object Reference"))
  (bind _unit_temp (`local.Unit_Temp`))
  (bind _result (`BlueprintSetLibrary.Set_ToArray` (`.UnitSet_3_262A6420454D014985B48BB0353FFCB7` (break `/Game/TurnBasedGame/Blueprints/Battle/Utilities/BPS_UnitSet` (`BlueprintMapLibrary.Map_Find` (`/Game/TurnBasedGame/Blueprints/Battle/BP_Battle.UnitTeams` (`self.Battle`)) (`/Game/TurnBasedGame/Blueprints/Unit/BP_Unit.TeamIndex` (`self.Unit`)))))))
  ;[1 1 1] check only for living units in the same team by iterating over a unit set. check if self is included and return resulting array.
  (for _array_element _result
    (set `local.Unit_Temp` _array_element)
    (if (`/Game/TurnBasedGame/Blueprints/Unit/BP_Unit.IsAlive` (`local.Unit_Temp`))
      (if (or (!= (`local.Unit_Temp`) (`self.Unit`)) (`local.IsSelfIncluded`))
        (`BlueprintMapLibrary.Map_Add` (`local.ReturnUnits`) (`/Game/TurnBasedGame/Blueprints/Unit/BP_Unit.Index` _unit_temp) _unit_temp))))
  (return (`local.ReturnUnits`)))

(fn `AIGetCastableSpells`
  (returns (Spells :type "Array of /Game/TurnBasedGame/Blueprints/Battle/Spells/Utilities/BPS_SpellData Structure"))
  (locals (ReturnSpell :type "Array of /Game/TurnBasedGame/Blueprints/Battle/Spells/Utilities/BPS_SpellData Structure"))
  (bind _unit (`self.Unit`))
  ;[1 1 1] loop over all castable spells to return an array
  (for _array_element (`.AvailableSpells_22_B8E89C4A46E2713CC7D8EEACAC0A8795` (break `/Game/TurnBasedGame/Blueprints/Unit/Utilities/BPS_Unit_Stats` (`.Stats_8_59677AC742C58E50C0B0B8BFC3DDDE60` (break `/Game/TurnBasedGame/Blueprints/Unit/Utilities/BPS_Unit` (`/Game/TurnBasedGame/Blueprints/Unit/BP_Unit.UnitData` _unit)))))
    (bind _spelldata (`/Game/TurnBasedGame/Blueprints/Battle/Spells/Utilities/BFL_Spells.GetSpellDataFromSpell` _array_element))
    (bind _cancast (`/Game/TurnBasedGame/Blueprints/Unit/BP_Unit.CanCastSpell` _unit _spelldata))
    (if _cancast
      (`KismetArrayLibrary.Array_Add` (`local.ReturnSpell`) _spelldata)))
  (return (`local.ReturnSpell`)))

(fn `AIGetEnemyUnits`
  (params (TeamIndexes :type "Array of Integer"))
  (returns (Units :type "Map of IntPoint Structure to /Game/TurnBasedGame/Blueprints/Unit/BP_Unit Object Reference"))
  (locals (ReturnUnits :type "Map of IntPoint Structure to /Game/TurnBasedGame/Blueprints/Unit/BP_Unit Object Reference") (Teams :type "Array of Integer") (Unit_Temp :type "/Game/TurnBasedGame/Blueprints/Unit/BP_Unit Object Reference"))
  (bind _unit_temp (`local.Unit_Temp`))
  (if (> (`KismetArrayLibrary.Array_Length` TeamIndexes) 0)
    (set `local.Teams` (`local.TeamIndexes`))
    (else
      (bind _keys (`BlueprintMapLibrary.Map_Keys` (`/Game/TurnBasedGame/Blueprints/Battle/BP_Battle.UnitTeams` (`self.Battle`))))
      (set `local.Teams` _keys)))
  ;[1 1 1] analogous to the unit blueprint, iterate over all living units that are not in the own team and return them as array
  (`KismetArrayLibrary.Array_RemoveItem` (`local.Teams`) (`/Game/TurnBasedGame/Blueprints/Unit/BP_Unit.TeamIndex` (`self.Unit`)))
  (for _array_element (`local.Teams`)
    (bind _result (`BlueprintSetLibrary.Set_ToArray` (`.UnitSet_3_262A6420454D014985B48BB0353FFCB7` (break `/Game/TurnBasedGame/Blueprints/Battle/Utilities/BPS_UnitSet` (`BlueprintMapLibrary.Map_Find` (`/Game/TurnBasedGame/Blueprints/Battle/BP_Battle.UnitTeams` (`self.Battle`)) _array_element)))))
    (for _array_element_2 _result
      (set `local.Unit_Temp` _array_element_2)
      (if (`/Game/TurnBasedGame/Blueprints/Unit/BP_Unit.IsAlive` (`local.Unit_Temp`))
        (`BlueprintMapLibrary.Map_Add` (`local.ReturnUnits`) (`/Game/TurnBasedGame/Blueprints/Unit/BP_Unit.Index` _unit_temp) _unit_temp))))
  (return (`local.ReturnUnits`)))

(fn `AIGetPathfinding`
  (returns (Pathfinding :type "/Game/TurnBasedGame/Blueprints/Grid/BP_Pathfinding Object Reference"))
  ;[1 1 1] help method for getting the pathfinding for ai via battle instance.
  (return (`/Game/TurnBasedGame/Blueprints/Grid/BP_Grid.GridPathfinding_AI` (`/Game/TurnBasedGame/Blueprints/Battle/BP_Battle.Grid` (`self.Battle`)))))

(fn `AIGetPathWithoutReachableTiles`
  (params (Target :type "IntPoint Structure"))
  (returns (Path :type "Array of IntPoint Structure"))
  (bind ((`ValidTileTypes_6_15FC62644524545BA5E30EA063EF24D4` _validtiletypes) (`CanMoveDiagonal_4_93F482A44F4F1FD66CC945895CDB6EDC` _canmovediagonal) (`MP_Current_9_342C6130430EBE8DE80D35B13735B31E` _mp_current)) (break `/Game/TurnBasedGame/Blueprints/Unit/Utilities/BPS_Unit_Stats` (`.Stats_8_59677AC742C58E50C0B0B8BFC3DDDE60` (break `/Game/TurnBasedGame/Blueprints/Unit/Utilities/BPS_Unit` (`/Game/TurnBasedGame/Blueprints/Unit/BP_Unit.UnitData` (`self.Unit`))))))
  (bind _path (`/Game/TurnBasedGame/Blueprints/Grid/BP_Pathfinding.FindPath` (`self.AIGetPathfinding`) (`/Game/TurnBasedGame/Blueprints/Unit/BP_Unit.Index` (`self.Unit`)) Target _canmovediagonal _validtiletypes 0.1 10.0 false _mp_current))
  (return _path))

(fn `AIGetPathWithReachableTiles`
  (returns (Path :type "Array of IntPoint Structure"))
  (bind _unit (`self.Unit`))
  (bind ((`ValidTileTypes_6_15FC62644524545BA5E30EA063EF24D4` _validtiletypes) (`CanMoveDiagonal_4_93F482A44F4F1FD66CC945895CDB6EDC` _canmovediagonal) (`MP_Current_9_342C6130430EBE8DE80D35B13735B31E` _mp_current)) (break `/Game/TurnBasedGame/Blueprints/Unit/Utilities/BPS_Unit_Stats` (`.Stats_8_59677AC742C58E50C0B0B8BFC3DDDE60` (break `/Game/TurnBasedGame/Blueprints/Unit/Utilities/BPS_Unit` (`/Game/TurnBasedGame/Blueprints/Unit/BP_Unit.UnitData` _unit)))))
  (bind _path (`/Game/TurnBasedGame/Blueprints/Grid/BP_Pathfinding.FindPath` (`self.AIGetPathfinding`) (`/Game/TurnBasedGame/Blueprints/Unit/BP_Unit.Index` _unit) (make `IntPoint` -999 -999) _canmovediagonal _validtiletypes 0.1 10.0 true _mp_current))
  (return _path))

(fn `AIGetUnitMoveLogic`
  (returns (MoveLogic :type "/Game/TurnBasedGame/Blueprints/AI/E_AIMoveLogic Enum"))
  ;[1 1 1] help method for getting the ai move logic of the unit as defined in data table.
  (return (`.MoveLogic_3_62F7D5D245AE408CA77214898E15561E` (break `/Game/TurnBasedGame/Blueprints/Unit/Utilities/BPS_Unit_AI` (`.AI_14_6A2A83F24282206CF593D6B8B74928C2` (break `/Game/TurnBasedGame/Blueprints/Unit/Utilities/BPS_Unit` (`/Game/TurnBasedGame/Blueprints/Unit/BP_Unit.UnitData` (`self.Unit`))))))))

(fn `AIGetUnitsInBattle`
  (params (IncludeSelf :type Boolean))
  (returns (AllUnits :type "Map of IntPoint Structure to /Game/TurnBasedGame/Blueprints/Unit/BP_Unit Object Reference"))
  (locals (ReturnUnits :type "Map of IntPoint Structure to /Game/TurnBasedGame/Blueprints/Unit/BP_Unit Object Reference") (UnitTemp :type "/Game/TurnBasedGame/Blueprints/Unit/BP_Unit Object Reference"))
  (bind _unittemp (`local.UnitTemp`))
  (for _array_element (`/Game/TurnBasedGame/Blueprints/Battle/BP_Battle.UnitsInBattle` (`self.Battle`))
    (set `local.UnitTemp` _array_element)
    (if (`/Game/TurnBasedGame/Blueprints/Unit/BP_Unit.IsAlive` (`local.UnitTemp`))
      (if (or (!= (`local.UnitTemp`) (`self.Unit`)) (`local.IncludeSelf`))
        (`BlueprintMapLibrary.Map_Add` (`local.ReturnUnits`) (`/Game/TurnBasedGame/Blueprints/Unit/BP_Unit.Index` _unittemp) _unittemp))))
  (return (`local.ReturnUnits`)))

(fn `AIImpactScoreHandler`
  (params (Spell :type "/Game/TurnBasedGame/Blueprints/Battle/Spells/Utilities/BPS_SpellData Structure") (AttackedUnit :type "/Game/TurnBasedGame/Blueprints/Unit/BP_Unit Object Reference"))
  (returns (ImpactScore :type "Float (double-precision)"))
  (locals (ApCost :type "Float (double-precision)") (IsAlly :type Boolean) (HpScore :type "Float (double-precision)"))
  (`|ExecutionSequence`
    (:`then_0`
      ;[1 1 1] save the ap cost by multiplying the actual cost of the spell with a factor.
      (bind _returnvalue (`self.AICalculateApCost` (struct)))
      (set `local.ApCost` _returnvalue)
      ;[1 1 1] check if the attacked unit is on the same team as the casting unit.
      (set `local.IsAlly` (== (`/Game/TurnBasedGame/Blueprints/Unit/BP_Unit.TeamIndex` (`self.Unit`)) (`/Game/TurnBasedGame/Blueprints/Unit/BP_Unit.TeamIndex` (`local.AttackedUnit`))))
      ;[1 1 1] calculate the hp score. if the target is an ally and the spell deals damage, multiply the score by -1 to show the negative outcome. if the target is an ally and the spell heals, multiply by 1. switch this behaviour if the target is an enemy. the hp value is a changable factor that can give this calculation more value.
      (bind _score (`self.AICalculateHpScore` (`local.Spell`) (`local.AttackedUnit`) (`local.IsAlly`)))
      (set `local.HpScore` _score)
      ;[1 1 1] calculate the killing blow score. give the killing blow of a unit the highest possible value. try to factor in the possible killing of allied units with area of effect spells.
      (bind _killingblowscore (`self.AICalculateKillingBlowScore` (`local.Spell`) (`local.AttackedUnit`) (`local.IsAlly`)))
      (set `self.KillingBlowScore` _killingblowscore))
    (:`then_1`
      ;[1 1 1] impact score gets calculated by adding up the hp score and killing blow score and dividing it by the maximum of either the calculated cost or 1 (so no division by zero).
      (return (/ (+ (`local.HpScore`) 0.0) (`KismetMathLibrary.FMax` (`local.ApCost`) 1.0))))))

(fn `AISpellCastHandler`
  (params (Target :type "IntPoint Structure") (Origin :type "IntPoint Structure") (Spell :type "/Game/TurnBasedGame/Blueprints/Battle/Spells/Utilities/BPS_SpellData Structure"))
  (locals (AllUnitsWithoutSelf :type "Map of IntPoint Structure to /Game/TurnBasedGame/Blueprints/Unit/BP_Unit Object Reference") (AttackedIndexes :type "Array of IntPoint Structure") (Score :type "Float (double-precision)") (AttackedIndex :type "IntPoint Structure") (AttackedUnit :type "/Game/TurnBasedGame/Blueprints/Unit/BP_Unit Object Reference") (DistanceOffset :type "Float (double-precision)" :default -0.0001))
  (bind _allunits (`self.AIGetUnitsInBattle` false))
  (set `local.AllUnitsWithoutSelf` _allunits)
  (bind _attackedindexes (`/Game/TurnBasedGame/Blueprints/Battle/BP_Battle.GetAttackedIndexes` (`self.Battle`) (`local.Target`) (`local.Spell`)))
  (set `local.AttackedIndexes` _attackedindexes)
  ;[1 1 1] the further away the unit to attack is, the lower the inital score gets by multiplying the distance with the negative distance offset. alter to give the distance more value.
  (set `local.Score` (* (`KismetMathLibrary.Distance2D` (`KismetMathLibrary.Conv_IntPointToVector2D` (`/Game/TurnBasedGame/Blueprints/Unit/BP_Unit.Index` (`self.Unit`))) (`KismetMathLibrary.Conv_IntPointToVector2D` (`local.Origin`))) (`local.DistanceOffset`)))
  ;[1 1 1] loop through all attacked tiles to add all scores. mainly used for area of effect spells.
  (for _array_element (`local.AttackedIndexes`)
    (set `local.AttackedIndex` _array_element)
    ;[1 1 1] if attacked index equals origin, the target is self. this can be used for heals or other area of effect abilities cast on self.
    (if (`KismetMathLibrary.Equal_IntPointIntPoint` (`local.AttackedIndex`) (`local.Origin`))
      (set `local.AttackedUnit` (`self.Unit`))
      (else
        (set `local.AttackedUnit` (`BlueprintMapLibrary.Map_Find` (`local.AllUnitsWithoutSelf`) (`local.AttackedIndex`)))))
    (`/Engine/EditorBlueprintResources/StandardMacros.IsValid` (`local.AttackedUnit`)
      (:`Is Valid`
        ;[1 1 1] add up the impact of the spell to get the impact score.
        (bind _impactscore (`self.AIImpactScoreHandler` (`local.Spell`) (`local.AttackedUnit`)))
        (set `local.Score` (+ _impactscore (`local.Score`))))))
  ;[1 1 1] save the result by making a dedicated structure of spell, origin, target and score if the score is greater then a already saved score. used to determine the best possible spell.
  (if (> (`local.Score`) (`.SpellScore_13_B46B9C4643C2A3058DEB9A9335F5D0CB` (break `/Game/TurnBasedGame/Blueprints/AI/S_UnitAISpellCastData` (`self.AISpellCast`))))
    (set `self.AISpellCast` (make `/Game/TurnBasedGame/Blueprints/AI/S_UnitAISpellCastData` true (`.Spell_4_BE14505B4C6395A0D6DC359116D559E2` (break `/Game/TurnBasedGame/Blueprints/Battle/Spells/Utilities/BPS_SpellData` (`local.Spell`))) (`local.Origin`) (`local.Target`) (`local.Score`)))))

(fn `AIStatScoreHandler`
  (params (ImpactMinMax :type "IntPoint Structure (by ref)") (IsAlly :type Boolean))
  (returns (Score :type "Float (double-precision)"))
  (bind (_x _y) (break `IntPoint` ImpactMinMax))
  (bind _returnvalue (/ (+ _x _y) 2))
  (return (* (`KismetMathLibrary.SelectFloat` 1.0 -1.0 (== (> _returnvalue 0) (`local.IsAlly`))) (`KismetMathLibrary.Abs` (* _returnvalue (`self.HpValue`))))))

(fn `UserConstructionScript`)