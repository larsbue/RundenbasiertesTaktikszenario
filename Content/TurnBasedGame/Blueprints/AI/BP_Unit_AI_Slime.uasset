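; Slime unit AI for the turn-based game, a child Blueprint that varies its move logic by whether it has attacked this turn.
; It clears a damage flag at turn start and sets it when a cast spell's HP modifier X value is negative.
; The move logic override returns a different enum value once that flag is set.
; Other battle hooks simply call the parent implementation.
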(event `self.CastSelectedSpell`
  (bind _spelldata (`/Game/TurnBasedGame/Blueprints/Battle/Spells/Utilities/BFL_Spells.GetSpellDataFromSpell` (`.Spell_7_616A2B6D4F75A9B154D92CA70508ACB2` (break `/Game/TurnBasedGame/Blueprints/AI/S_UnitAISpellCastData` (`self.AISpellCast`)))))
  (set `self.DamageDoneThisTurn` (or (`self.DamageDoneThisTurn`) (< (`.X` (break `IntPoint` (`.MinMaxModifier_Hp_2_337387544FC677D17537229603DB65D4` (break `/Game/TurnBasedGame/Blueprints/Battle/Spells/Utilities/BPS_SpellData_Stats` (`.Stats_15_29A51BF842020762CC2E1FB71554CF3D` (break `/Game/TurnBasedGame/Blueprints/Battle/Spells/Utilities/BPS_SpellData` _spelldata)))))) 0)))
  (`parent.CastSelectedSpell`))

(fn `AIBattleEnded`
  (`parent.AIBattleEnded`))

(fn `AIBattleStarted`
  (`parent.AIBattleStarted`))

(fn `AIBeginTurn`
  (set `self.DamageDoneThisTurn` false)
  (`parent.AIBeginTurn`))

(fn `AIGetUnitMoveLogic`
  (returns (MoveLogic :type "/Game/TurnBasedGame/Blueprints/AI/E_AIMoveLogic Enum"))
  (return (select `bool` (`self.DamageDoneThisTurn`) :`false` "NewEnumerator0" :`true` "NewEnumerator2" :!type "/Game/TurnBasedGame/Blueprints/AI/E_AIMoveLogic Enum")))

(fn `UserConstructionScript`
  (`parent.UserConstructionScript`))