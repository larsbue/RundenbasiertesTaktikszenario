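; BP_SpellAnims is an actor that plays a grid-based spell's animation across all attacked tiles.
; On BeginPlay it spawns one BP_SpellAnim per attacked index, animating the grid's tile mesh from the origin tile to that target with randomized red brightness and play rate.
; Each finished shape fires a hit event and removes its index.
; When none remain, it signals completion and destroys itself.
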(event `self.ReceiveBeginPlay`
  (`self.PlaySpellAnimation`))

(event `PlaySpellAnimation`
  (bind (_transform_location _transform_rotation) (`KismetMathLibrary.BreakTransform` (`self.Tranform` (`self.OriginIndex`))))
  (bind ((`Mesh_5_8018674F4F2F06D91A959FAC3401F4D6` _mesh) (`MeshMaterial_8_6B4B373D44D77511B854CEA336BC2031` _meshmaterial)) (break `/Game/TurnBasedGame/Blueprints/Grid/GridRessources/S_DataGridShape` (`/Game/TurnBasedGame/Blueprints/Grid/BP_Grid.GetGridShapeData` (`self.Grid`))))
  (for _array_element (`self.AttackedIndexes`)
    (bind _returnvalue (`|SpawnActorFromClass` "/Game/TurnBasedGame/Blueprints/Combat/Spells/SpellAnims/BP_SpellAnim.BP_SpellAnim_C" (`KismetMathLibrary.MakeTransform` (0.0 0.0 0.0)) "AlwaysSpawn" "MultiplyWithRoot" null _mesh _meshmaterial (* (struct :`R` 1.0 :`A` 1.0) (`KismetMathLibrary.RandomFloatInRange` 0.25 1.75)) (`KismetMathLibrary.MakeTransform` _transform_location _transform_rotation (0.01 0.01 0.01)) (`self.Tranform` _array_element) (`KismetMathLibrary.RandomFloatInRange` 0.75 1.25) _array_element null))
    (add `/Game/TurnBasedGame/Blueprints/Combat/Spells/SpellAnims/BP_SpellAnim.OnShapeAnimationCompleted` _returnvalue (delegate `OnShapeAnimationCompleted`))))

(event `OnShapeAnimationCompleted`
  (params (AnimatedShape :type "/Game/TurnBasedGame/Blueprints/Combat/Spells/SpellAnims/BP_SpellAnim Object Reference"))
  (bind _index (`/Game/TurnBasedGame/Blueprints/Combat/Spells/SpellAnims/BP_SpellAnim.Index` AnimatedShape))
  (bind _attackedindexes (`self.AttackedIndexes`))
  (`self.OnSpellAnimationHit` self _index)
  (`KismetArrayLibrary.Array_RemoveItem` _attackedindexes _index)
  (if (== (`KismetArrayLibrary.Array_Length` _attackedindexes) 0)
    (`self.CompleteSpellAnimation`)))

(event `CompleteSpellAnimation`
  (`self.OnSpellAnimationCompleted` self)
  (`self.K2_DestroyActor`))

(fn `Tranform`
  (params (Key :type "IntPoint Structure (by ref)"))
  (returns (Transform :type "Transform Structure"))
  (return (`.Transform_8_4368262E41BF048BC408BDB4D4AEF3EB` (break `/Game/TurnBasedGame/Blueprints/Grid/Utilities/S_DataTile` (`BlueprintMapLibrary.Map_Find` (`/Game/TurnBasedGame/Blueprints/Grid/BP_Grid.GridTiles` (`self.Grid`)) Key)))))

(fn `UserConstructionScript`)