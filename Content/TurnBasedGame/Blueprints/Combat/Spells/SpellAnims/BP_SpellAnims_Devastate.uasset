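; Spell animation actor for Devastate in the turn-based combat system, playing a sword slash from the caster's tile toward the target.
; It places itself at the origin index facing the target index, then a timeline drives the pitch and scale of its Animation component.
; Once playback passes a set point, it fires the hit callback for the target through a DoOnce, then completes the spell animation when the timeline finishes.
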(event `self.PlaySpellAnimation`
  (bind _animation (`self.Animation`))
  (bind _transform_location (`KismetMathLibrary.BreakTransform` (`self.Tranform` (`self.OriginIndex`))))
  (`self.K2_SetActorLocationAndRotation` _transform_location (`KismetMathLibrary.FindLookAtRotation` (`KismetMathLibrary.Conv_Vector2DToVector` (`KismetMathLibrary.Conv_IntPointToVector2D` (`self.OriginIndex`))) (`KismetMathLibrary.Conv_Vector2DToVector` (`KismetMathLibrary.Conv_IntPointToVector2D` (`self.TargetIndex`)))))
  (bind (_direction _rotationy _scale) (`Timeline|Timeline_SwordSlash` :!via `PlayFromStart`)
    (:`Update`
      (`SceneComponent.K2_SetRelativeRotation` _animation (`KismetMathLibrary.MakeRotator` 0.0 _rotationy) false false)
      (`SceneComponent.SetRelativeScale3D` _animation (`KismetMathLibrary.Conv_DoubleToVector` _scale))
      (if (>= (`TimelineComponent.GetPlaybackPosition` (`self.Timeline_SwordSlash`)) 0.4)
        (`/Engine/EditorBlueprintResources/StandardMacros.DoOnce` false
          (:`Completed`
            (`self.OnSpellAnimationHit` self (`self.TargetIndex`))))))
    (:`Finished`
      (`self.CompleteSpellAnimation`))))

(fn `UserConstructionScript`
  (`parent.UserConstructionScript`))