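; Spell animation actor for Arrow Rain that flies its Animation component from the origin index to the target index in the turn-based combat.
; On play it faces the target, then a timeline drives position interpolation, height offset, pitch and scale.
; A DoOnce fires the hit callback for the target index at a fixed playback time, and the timeline's end completes the spell animation.
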(event `self.PlaySpellAnimation`
  (bind _animation (`self.Animation`))
  (bind _transform_location (`KismetMathLibrary.BreakTransform` (`self.Tranform` (`self.OriginIndex`))))
  (bind _transform_location_2 (`KismetMathLibrary.BreakTransform` (`self.Tranform` (`self.OriginIndex`))))
  (bind _transform_location_3 (`KismetMathLibrary.BreakTransform` (`self.Tranform` (`self.TargetIndex`))))
  (`self.K2_SetActorLocationAndRotation` _transform_location_2 (`KismetMathLibrary.FindLookAtRotation` (`KismetMathLibrary.Conv_Vector2DToVector` (`KismetMathLibrary.Conv_IntPointToVector2D` (`self.OriginIndex`))) (`KismetMathLibrary.Conv_Vector2DToVector` (`KismetMathLibrary.Conv_IntPointToVector2D` (`self.TargetIndex`)))))
  (bind (_direction _rotationy _scale _locationz _locationalpha) (`Timeline|Timeline_Arrow` :!via `PlayFromStart`)
    (:`Update`
      (`self.K2_SetActorLocation` (+ (`KismetMathLibrary.VLerp` _transform_location _transform_location_3 _locationalpha) (`KismetMathLibrary.MakeVector` 0.0 0.0 _locationz)))
      (`SceneComponent.K2_SetRelativeRotation` _animation (`KismetMathLibrary.MakeRotator` 0.0 _rotationy) false false)
      (`SceneComponent.SetRelativeScale3D` _animation (`KismetMathLibrary.Conv_DoubleToVector` _scale))
      (if (>= (`TimelineComponent.GetPlaybackPosition` (`self.Timeline_Arrow`)) 0.3)
        (`/Engine/EditorBlueprintResources/StandardMacros.DoOnce` false
          (:`Completed`
            (`self.OnSpellAnimationHit` self (`self.TargetIndex`))))))
    (:`Finished`
      (`self.CompleteSpellAnimation`))))

(fn `UserConstructionScript`
  (`parent.UserConstructionScript`))