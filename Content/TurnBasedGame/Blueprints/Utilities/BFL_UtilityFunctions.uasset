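; Blueprint function library of small math helpers for the turn-based game.
; It snaps a vector to a per-axis grid size and tests whether floats or integers are even.
; MinMaxRandom rolls an integer between two bounds in either order, so one call handles both positive heal and negative damage ranges.
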(fn `isFloatEven`
  (params (Float :type "Float (double-precision)"))
  (returns (IsEven :type Boolean))
  (return (== (mod Float 2.0) 0.0)))

(fn `isIntEven`
  (params (Int :type Integer) (__WorldContext :type "Object Object Reference"))
  (returns (IsEven :type Boolean))
  (return (== (mod Int 2) 0)))

(fn `MinMaxRandom`
  (params (MinMax :type "IntPoint Structure"))
  (returns (Output :type Integer))
  (bind (_minmax_x _minmax_y) (break `IntPoint` (`local.MinMax`)))
  (bind (_minmax_x_2 _minmax_y_2) (break `IntPoint` (`local.MinMax`)))
  ;[1 1 1] returns a random integer between x and y. normal for heal, reverse for damage (because negative).
  (if (<= MinMax_X MinMax_Y)
    (return (`KismetMathLibrary.RandomIntegerInRange` _minmax_x_2 _minmax_y_2))
    (else
      (return (`KismetMathLibrary.RandomIntegerInRange` _minmax_y _minmax_x)))))

(fn `SnapVectorToVector`
  (params (V1 :type "Vector Structure") (V2 :type "Vector Structure"))
  (returns (Return :type "Vector Structure"))
  (return (`KismetMathLibrary.MakeVector` (`KismetMathLibrary.GridSnap_Float` V1_X V2_X) (`KismetMathLibrary.GridSnap_Float` V1_Y V2_Y) (`KismetMathLibrary.GridSnap_Float` V1_Z V2_Z))))