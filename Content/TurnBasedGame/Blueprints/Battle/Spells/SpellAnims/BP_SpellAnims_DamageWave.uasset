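; Turn-based battle spell animation for a purple dark damage wave, placed at the target index's transform.
; A timeline scales the wave and feeds its opacity track to three meshes' materials, though the scalar parameter name is None.
; Once playback reaches 0.1 seconds, a DoOnce fires the hit callback for every attacked index, and the timeline's end completes the animation.
; The construction script tints the meshes in three shades of purple.
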(event `self.PlaySpellAnimation`
  (bind _transform_location (`KismetMathLibrary.BreakTransform` (`self.Tranform` (`self.TargetIndex`))))
  (`self.K2_SetActorLocation` _transform_location)
  (bind (_direction _scale _opacity) (`Timeline|Timeline_DarkWave` :!via `PlayFromStart`)
    (:`Update`
      (`SceneComponent.SetRelativeScale3D` (`self.Animation_Scale`) _scale)
      (`MeshComponent.SetScalarParameterValueOnMaterials` (`self.StaticMesh`) "None" _opacity)
      (`MeshComponent.SetScalarParameterValueOnMaterials` (`self.StaticMesh1`) "None" _opacity)
      (`MeshComponent.SetScalarParameterValueOnMaterials` (`self.StaticMesh2`) "None" _opacity)
      (if (>= (`TimelineComponent.GetPlaybackPosition` (`self.Timeline_DarkWave`)) 0.1)
        (`/Engine/EditorBlueprintResources/StandardMacros.DoOnce` false
          (:`Completed`
            (for _array_element (`self.AttackedIndexes`)
              (`self.OnSpellAnimationHit` self _array_element))))))
    (:`Finished`
      (`self.CompleteSpellAnimation`))))

(fn `UserConstructionScript`
  (`parent.UserConstructionScript`)
  (`MeshComponent.SetVectorParameterValueOnMaterials` (`self.StaticMesh`) "Color" (`KismetMathLibrary.Conv_LinearColorToVector` (struct :`R` 0.404823 :`B` 1.0 :`A` 1.0)))
  (`MeshComponent.SetVectorParameterValueOnMaterials` (`self.StaticMesh2`) "Color" (`KismetMathLibrary.Conv_LinearColorToVector` (struct :`R` 0.253014 :`B` 0.625 :`A` 1.0)))
  (`MeshComponent.SetVectorParameterValueOnMaterials` (`self.StaticMesh1`) "Color" (`KismetMathLibrary.Conv_LinearColorToVector` (struct :`R` 0.134941 :`B` 0.333333 :`A` 1.0))))