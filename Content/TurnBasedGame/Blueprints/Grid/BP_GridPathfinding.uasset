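; A* pathfinder for the turn-based grid that returns either a path or the tiles reachable within a cost limit.
; Neighbors are filtered by tile type, occupancy and height step, then queued in a cost-sorted open list that breaks ties toward straight moves.
; Searches run instantly or spread over frames through a gated retriggerable delay and per-frame millisecond budget, reporting progress and results through callbacks.
; Only square grids are handled.
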(event `FindPathWithDelay`
  (`|ExecutionSequence`
    (:`then_0`
      (goto _label_3 :!via `Open`))
    (:`then_1`
      (set `self.LoopStartTime` (`KismetMathLibrary.Now`) :!label _label)
      (if (> (`KismetArrayLibrary.Array_Length` (`self.DiscoveredTileIndexes`)) 0) :!label _label_2
        (bind _foundtargettile (`self.AnalyseNextDiscoveredTile`))
        (if _foundtargettile
          (bind _path (`self.GeneratePath`))
          (`self.OnPathfindingCompleted` _path)
          (else
            (if (> (`self.MaxMsPerFrame`) 0.0)
              (if (< (- (`KismetMathLibrary.GetMillisecond` (`KismetMathLibrary.Now`)) (`KismetMathLibrary.GetMillisecond` (`self.LoopStartTime`))) (`self.MaxMsPerFrame`))
                (goto _label_2)
                (else
                  _)))
            (`KismetSystemLibrary.RetriggerableDelay` (`self.DelayBetweenIterations`))
            (`/Engine/EditorBlueprintResources/StandardMacros.Gate` true :!label _label_3
              (:`Exit`
                (goto _label)))))
        (else
          (`self.OnPathfindingCompleted` (select `bool` (`self.ReturnReachableTiles`) :`false` (`|MakeArray`) :`true` (`self.AnalysedTileIndexes`))))))))

(event `CloseDelayGate`
  (goto _label_3 :!via `Close`))

(fn `AnalyseNextDiscoveredTile`
  (returns (FoundTargetTile :type Boolean))
  (bind _tilepathdata (`self.PullCheapestTileOutOfTheDiscoveredList`))
  (bind _output_get (set `self.CurrentDiscoveredTile` _tilepathdata))
  (`self.OnPathfindingDataUpdated` (`.Index_6_2F955D2D4AD0190907C32EAE2D9351BE` (break `/Game/TurnBasedGame/Blueprints/Grid/Utilities/S_DataPathfinding` _output_get)))
  (bind _neighbors (`self.GetValidTileNeighbors` (`.Index_6_2F955D2D4AD0190907C32EAE2D9351BE` (break `/Game/TurnBasedGame/Blueprints/Grid/Utilities/S_DataPathfinding` (`self.CurrentDiscoveredTile`))) (`self.IncludeDiagonals`) (`self.ValidTileTypes`)))
  (set `self.CurrentNeighbors` _neighbors)
  (while (> (`KismetArrayLibrary.Array_Length` (`self.CurrentNeighbors`)) 0)
    (bind _istargettile (`self.DiscoverNextNeighbor`))
    (if _istargettile
      (return true)))
  (return false))

(fn `ClearGeneratedData`
  (`BlueprintMapLibrary.Map_Clear` (`self.DataPathfinding`))
  (`KismetArrayLibrary.Array_Clear` (`self.DiscoveredTileSortingCosts`))
  (`KismetArrayLibrary.Array_Clear` (`self.DiscoveredTileIndexes`))
  (`KismetArrayLibrary.Array_Clear` (`self.AnalysedTileIndexes`))
  (`self.OnPathfindingDataCleared`))

(fn `DiscoverNextNeighbor`
  (returns (IsTargetTile :type Boolean))
  (locals (CostFromStart :type Integer) (IndexInDiscovered :type Integer :default 0))
  (bind _indexindiscovered (`local.IndexInDiscovered`))
  (bind (_index _costtoentertile) (break `/Game/TurnBasedGame/Blueprints/Grid/Utilities/S_DataPathfinding` (`self.CurrentNeigbor`)))
  (set `self.CurrentNeigbor` (`|GetArrayItem` (`self.CurrentNeighbors`)))
  (`KismetArrayLibrary.Array_Remove` (`self.CurrentNeighbors`))
  (if (not (`KismetArrayLibrary.Array_Contains` (`self.AnalysedTileIndexes`) (`.Index_6_2F955D2D4AD0190907C32EAE2D9351BE` (break `/Game/TurnBasedGame/Blueprints/Grid/Utilities/S_DataPathfinding` (`self.CurrentNeigbor`)))))
    (set `local.CostFromStart` (+ (`.CostFromStart_11_EA5427FC41E2C191DAB85F96CEF5C798` (break `/Game/TurnBasedGame/Blueprints/Grid/Utilities/S_DataPathfinding` (`self.CurrentDiscoveredTile`))) (`.CostToEnterTIle_8_516C173A4F356563CF015EAB160915A8` (break `/Game/TurnBasedGame/Blueprints/Grid/Utilities/S_DataPathfinding` (`self.CurrentNeigbor`)))))
    (if (<= (`local.CostFromStart`) (`self.MaxPathLength`))
      (bind _output_get (set `local.IndexInDiscovered` (`KismetArrayLibrary.Array_Find` (`self.DiscoveredTileIndexes`) (`.Index_6_2F955D2D4AD0190907C32EAE2D9351BE` (break `/Game/TurnBasedGame/Blueprints/Grid/Utilities/S_DataPathfinding` (`self.CurrentNeigbor`))))))
      (if (not (== _output_get -1))
        (bind _output_get_2 (set `self.CurrentNeigbor` (`BlueprintMapLibrary.Map_Find` (`self.DataPathfinding`) (`.Index_6_2F955D2D4AD0190907C32EAE2D9351BE` (break `/Game/TurnBasedGame/Blueprints/Grid/Utilities/S_DataPathfinding` (`self.CurrentNeigbor`))))))
        (if (< (`local.CostFromStart`) (`.CostFromStart_11_EA5427FC41E2C191DAB85F96CEF5C798` (break `/Game/TurnBasedGame/Blueprints/Grid/Utilities/S_DataPathfinding` _output_get_2)))
          (`KismetArrayLibrary.Array_Remove` (`self.DiscoveredTileIndexes`) _indexindiscovered)
          (`KismetArrayLibrary.Array_Remove` (`self.DiscoveredTileSortingCosts`) _indexindiscovered)
          (else
            (return false))))
      (`self.DiscoverTile` (make `/Game/TurnBasedGame/Blueprints/Grid/Utilities/S_DataPathfinding` _index _costtoentertile (`local.CostFromStart`) (`self.GetMinimumCostBetweenTwoTiles` (`.Index_6_2F955D2D4AD0190907C32EAE2D9351BE` (break `/Game/TurnBasedGame/Blueprints/Grid/Utilities/S_DataPathfinding` (`self.CurrentNeigbor`))) (`self.TargetIndex`) (`self.IncludeDiagonals`)) (`.Index_6_2F955D2D4AD0190907C32EAE2D9351BE` (break `/Game/TurnBasedGame/Blueprints/Grid/Utilities/S_DataPathfinding` (`self.CurrentDiscoveredTile`)))))
      (if (`KismetMathLibrary.Equal_IntPointIntPoint` (`.Index_6_2F955D2D4AD0190907C32EAE2D9351BE` (break `/Game/TurnBasedGame/Blueprints/Grid/Utilities/S_DataPathfinding` (`self.CurrentNeigbor`))) (`self.TargetIndex`))
        (return true)
        (else
          (return false)))
      (else
        (return false)))
    (else
      (return false))))

(fn `DiscoverTile`
  (params (TilePathData :type "/Game/TurnBasedGame/Blueprints/Grid/Utilities/S_DataPathfinding Structure"))
  (bind _index (break `/Game/TurnBasedGame/Blueprints/Grid/Utilities/S_DataPathfinding` TilePathData))
  (`BlueprintMapLibrary.Map_Add` (`self.DataPathfinding`) _index TilePathData)
  (`self.InsertTileInDiscoveredArray` TilePathData)
  (`self.OnPathfindingDataUpdated` _index))

(fn `FindPath`
  (params (Start :type "IntPoint Structure") (Target :type "IntPoint Structure") (Diagonals :type Boolean) (TileTypes :type "Array of /Game/TurnBasedGame/Blueprints/Grid/Utilities/E_TypeTile Enum") (Delay :type "Float (double-precision)") (MaxMs :type "Float (double-precision)") (ReturnReachables :type Boolean) (PathLength :type Integer))
  (returns (Path :type "Array of IntPoint Structure"))
  (bind _array (`|MakeArray`))
  (bind _returnvalue (select `bool` (`self.ReturnReachableTiles`) :`false` (`|MakeArray`) :`true` (`self.AnalysedTileIndexes`)))
  (set `self.StartIndex` Start)
  (set `self.TargetIndex` Target)
  (set `self.IncludeDiagonals` Diagonals)
  (set `self.ValidTileTypes` TileTypes)
  (set `self.DelayBetweenIterations` Delay)
  (set `self.MaxMsPerFrame` MaxMs)
  (set `self.ReturnReachableTiles` ReturnReachables)
  (set `self.MaxPathLength` PathLength)
  (`self.CloseDelayGate`)
  (`self.ClearGeneratedData`)
  (bind _isvalid (`self.IsInputDataValid`))
  (if _isvalid
    (`self.DiscoverTile` (make `/Game/TurnBasedGame/Blueprints/Grid/Utilities/S_DataPathfinding` (`self.StartIndex`) 1 0 (`self.GetMinimumCostBetweenTwoTiles` (`self.StartIndex`) (`self.TargetIndex`) (`self.IncludeDiagonals`))))
    (if (<= (`self.DelayBetweenIterations`) 0.0)
      (while (> (`KismetArrayLibrary.Array_Length` (`self.DiscoveredTileIndexes`)) 0)
        (bind _foundtargettile (`self.AnalyseNextDiscoveredTile`))
        (if _foundtargettile
          (bind _path (`self.GeneratePath`))
          (`self.OnPathfindingCompleted` _path)
          (return _path)))
      (`self.OnPathfindingCompleted` _returnvalue)
      (return _returnvalue)
      (else
        (`self.FindPathWithDelay`)
        (return (`|MakeArray`))))
    (else
      (`self.OnPathfindingCompleted` _array)
      (return _array))))

(fn `GeneratePath`
  (returns (Path :type "Array of IntPoint Structure"))
  (locals (Current :type "IntPoint Structure") (InvertedPath :type "Array of IntPoint Structure") (Ret :type "Array of IntPoint Structure"))
  (set `local.Current` (`self.TargetIndex`))
  (while (!= (`local.Current`) (`self.StartIndex`))
    (`KismetArrayLibrary.Array_Add` (`local.InvertedPath`) (`local.Current`))
    (set `local.Current` (`.PreviousIndex_14_210005584F4E61313D5EA7B6D5691723` (break `/Game/TurnBasedGame/Blueprints/Grid/Utilities/S_DataPathfinding` (`BlueprintMapLibrary.Map_Find` (`self.DataPathfinding`) (`local.Current`))))))
  (bind (_arrayindex _arrayelement) (`/Engine/EditorBlueprintResources/StandardMacros.ReverseForEachLoop` (`local.InvertedPath`))
    (:`LoopBody`
      (`KismetArrayLibrary.Array_Add` (`local.Ret`) _arrayelement))
    (:`Completed`
      (return (`local.Ret`)))))

(fn `GetMinimumCostBetweenTwoTiles`
  (params (StartIndex :type "IntPoint Structure") (EndIndex :type "IntPoint Structure") (Diagonals :type Boolean))
  (returns (MinCost :type Integer))
  (bind (_returnvalue_x _returnvalue_y) (break `IntPoint` (- (`local.StartIndex`) (`local.EndIndex`))))
  (bind (_returnvalue_x_2 _returnvalue_y_2) (break `IntPoint` (- (`local.StartIndex`) (`local.EndIndex`))))
  (if (`local.Diagonals`)
    (return (`KismetMathLibrary.Max` (`KismetMathLibrary.Abs_Int` _returnvalue_x_2) (`KismetMathLibrary.Abs_Int` _returnvalue_y_2)))
    (else
      (return (+ (`KismetMathLibrary.Abs_Int` _returnvalue_x) (`KismetMathLibrary.Abs_Int` _returnvalue_y))))))

(fn `GetNeighborIndexes`
  (params (Index :type "IntPoint Structure") (IncludeDiagonals :type Boolean))
  (returns (Neighbors :type "Array of IntPoint Structure"))
  (switch `/Game/TurnBasedGame/Blueprints/Grid/GridRessources/E_GridShape` (`/Game/TurnBasedGame/Blueprints/Grid/BP_Grid.GridShape` (`self.Grid`))
    (:`NewEnumerator1`
      (return (`self.GetNeighborIndexesForSquare` (`local.Index`) (`local.IncludeDiagonals`))))))

(fn `GetNeighborIndexesForSquare`
  (params (Index :type "IntPoint Structure") (IncludeDiagonals :type Boolean))
  (returns (Neighbors :type "Array of IntPoint Structure"))
  (locals (Ret :type "Array of IntPoint Structure"))
  (bind _array (`|MakeArray` (+ (`local.Index`) (make `IntPoint` 1)) (+ (`local.Index`) (make `IntPoint` 0 1)) (+ (`local.Index`) (make `IntPoint` -1)) (+ (`local.Index`) (make `IntPoint` 0 -1))))
  (if IncludeDiagonals
    (set `local.Ret` _array)
    (`KismetArrayLibrary.Array_Append` (`local.Ret`) (`|MakeArray` (+ (`local.Index`) (make `IntPoint` 1 1)) (+ (`local.Index`) (make `IntPoint` -1 1)) (+ (`local.Index`) (make `IntPoint` -1 -1)) (+ (`local.Index`) (make `IntPoint` 1 -1))))
    (return (`local.Ret`))
    (else
      (return _array))))

(fn `GetPathCost`
  (params (Path :type "Array of IntPoint Structure"))
  (returns (Cost :type Integer))
  (locals (Return :type Integer))
  (set `local.Return` 0)
  (for _array_element (`local.Path`)
    (set `local.Return` (+ (`local.Return`) (`/Game/TurnBasedGame/Blueprints/Grid/Utilities/BFL_TileData.GetCostByTileType` (`.Type_6_5F1D582544258A461E8CED80E64FB436` (break `/Game/TurnBasedGame/Blueprints/Grid/Utilities/S_DataTile` (`BlueprintMapLibrary.Map_Find` (`/Game/TurnBasedGame/Blueprints/Grid/BP_Grid.GridTiles` (`self.Grid`)) _array_element)))))))
  (return (`local.Return`)))

(fn `GetTileSortingCost`
  (params (TileData :type "/Game/TurnBasedGame/Blueprints/Grid/Utilities/S_DataPathfinding Structure (by ref)"))
  (returns (Cost :type Integer))
  (bind (_index _costtoentertile _costfromstart _mincosttotarget _previousindex) (break `/Game/TurnBasedGame/Blueprints/Grid/Utilities/S_DataPathfinding` TileData))
  (bind (_index_2 _costtoentertile_2 _costfromstart_2 _mincosttotarget_2) (break `/Game/TurnBasedGame/Blueprints/Grid/Utilities/S_DataPathfinding` TileData))
  (return (+ (* (+ _costfromstart_2 _mincosttotarget_2) 2) (`self.IsDiagonal` _index _previousindex))))

(fn `GetValidTileNeighbors`
  (params (Index :type "IntPoint Structure") (IncludeDiagonals :type Boolean) (ValidTypes :type "Array of /Game/TurnBasedGame/Blueprints/Grid/Utilities/E_TypeTile Enum"))
  (returns (Neighbors :type "Array of /Game/TurnBasedGame/Blueprints/Grid/Utilities/S_DataPathfinding Structure"))
  (locals (Data :type "/Game/TurnBasedGame/Blueprints/Grid/Utilities/S_DataTile Structure") (InputData :type "/Game/TurnBasedGame/Blueprints/Grid/Utilities/S_DataTile Structure") (ReturnDataPathfinding :type "Array of /Game/TurnBasedGame/Blueprints/Grid/Utilities/S_DataPathfinding Structure"))
  (bind (_data_index _data_type) (break `/Game/TurnBasedGame/Blueprints/Grid/Utilities/S_DataTile` (`local.Data`)))
  (bind (_data_index_2 _data_type_2) (break `/Game/TurnBasedGame/Blueprints/Grid/Utilities/S_DataTile` (`local.Data`)))
  (bind (_data_index_3 _data_type_3 _data_transform _data_states _data_unitontile) (break `/Game/TurnBasedGame/Blueprints/Grid/Utilities/S_DataTile` (`local.Data`)))
  (bind (_gridtilesize_x _gridtilesize_y _gridtilesize_z) (`KismetMathLibrary.BreakVector` (`/Game/TurnBasedGame/Blueprints/Grid/BP_Grid.GridTileSize` (`self.Grid`))))
  (set `local.InputData` (`BlueprintMapLibrary.Map_Find` (`/Game/TurnBasedGame/Blueprints/Grid/BP_Grid.GridTiles` (`self.Grid`)) (`local.Index`)))
  (bind _neighbors (`self.GetNeighborIndexes` (`local.Index`) (`local.IncludeDiagonals`)))
  (for _array_element _neighbors
    (set `local.Data` (`BlueprintMapLibrary.Map_Find` (`/Game/TurnBasedGame/Blueprints/Grid/BP_Grid.GridTiles` (`self.Grid`)) _array_element))
    (if (`KismetArrayLibrary.Array_Contains` (`local.ValidTypes`) _data_type)
      (if (not (`KismetSystemLibrary.IsValid` _data_unitontile))
        (if (<= (`KismetMathLibrary.Abs` (- (.z (.location (`.Transform_8_4368262E41BF048BC408BDB4D4AEF3EB` (break `/Game/TurnBasedGame/Blueprints/Grid/Utilities/S_DataTile` (`local.Data`))))) (.z (.location (`.Transform_8_4368262E41BF048BC408BDB4D4AEF3EB` (break `/Game/TurnBasedGame/Blueprints/Grid/Utilities/S_DataTile` (`local.InputData`))))))) _gridtilesize_z)
          (`KismetArrayLibrary.Array_Add` (`local.ReturnDataPathfinding`) (make `/Game/TurnBasedGame/Blueprints/Grid/Utilities/S_DataPathfinding` _data_index_2 (`/Game/TurnBasedGame/Blueprints/Grid/Utilities/BFL_TileData.GetCostByTileType` _data_type_2) 999999 999999 (`local.Index`)))))))
  (return (`local.ReturnDataPathfinding`)))

(fn `InsertTileInDiscoveredArray`
  (params (TileData :type "/Game/TurnBasedGame/Blueprints/Grid/Utilities/S_DataPathfinding Structure"))
  (locals (SortingCost :type Integer))
  (bind _discoveredtilesortingcosts (`self.DiscoveredTileSortingCosts`))
  (set `local.SortingCost` (`self.GetTileSortingCost` TileData))
  (if (== (`KismetArrayLibrary.Array_Length` (`self.DiscoveredTileSortingCosts`)) 0)
    (`KismetArrayLibrary.Array_Add` (`self.DiscoveredTileSortingCosts`) (`local.SortingCost`) :!label _label)
    (`KismetArrayLibrary.Array_Add` (`self.DiscoveredTileIndexes`) (`.Index_6_2F955D2D4AD0190907C32EAE2D9351BE` (break `/Game/TurnBasedGame/Blueprints/Grid/Utilities/S_DataPathfinding` (`local.TileData`))))
    (elif (>= (`local.SortingCost`) (`|GetArrayItem` _discoveredtilesortingcosts (`KismetArrayLibrary.Array_LastIndex` _discoveredtilesortingcosts)))
      (goto _label)
      (else
        (for (_array_element _array_index) (`self.DiscoveredTileSortingCosts`)
          (if (>= _array_element (`local.SortingCost`))
            (`KismetArrayLibrary.Array_Insert` (`self.DiscoveredTileSortingCosts`) (`local.SortingCost`) _array_index)
            (`KismetArrayLibrary.Array_Insert` (`self.DiscoveredTileIndexes`) (`.Index_6_2F955D2D4AD0190907C32EAE2D9351BE` (break `/Game/TurnBasedGame/Blueprints/Grid/Utilities/S_DataPathfinding` (`local.TileData`))) _array_index)
            (break)))))))

(fn `IsDiagonal`
  (params (Index1 :type "IntPoint Structure") (Index2 :type "IntPoint Structure"))
  (returns (IsDiagonal :type Boolean))
  (bind _neighbors (`self.GetNeighborIndexes` Index1))
  (return (not (`KismetArrayLibrary.Array_Contains` _neighbors Index2))))

(fn `IsInputDataValid`
  (returns (IsValid :type Boolean))
  (bind ((`Type_6_5F1D582544258A461E8CED80E64FB436` _type) (`UnitOnTile_15_1E34864C4E787D0AB34915A28704B28C` _unitontile)) (break `/Game/TurnBasedGame/Blueprints/Grid/Utilities/S_DataTile` (`BlueprintMapLibrary.Map_Find` (`/Game/TurnBasedGame/Blueprints/Grid/BP_Grid.GridTiles` (`self.Grid`)) (`self.TargetIndex`))))
  (if (!= (`self.StartIndex`) (`self.TargetIndex`))
    (if (`/Game/TurnBasedGame/Blueprints/Grid/BP_Grid.IsTileWalkable` (`self.Grid`) (`self.StartIndex`))
      (if (not (`self.ReturnReachableTiles`))
        (if (`/Game/TurnBasedGame/Blueprints/Grid/BP_Grid.IsTileWalkable` (`self.Grid`) (`self.TargetIndex`))
          (if (<= (`self.GetMinimumCostBetweenTwoTiles` (`self.StartIndex`) (`self.TargetIndex`) (`self.IncludeDiagonals`)) (`self.MaxPathLength`))
            ;[1 1 1] check if the tile type of the target index is in valid tile types array and also check if the unit on the tile is valid.
            (if (`KismetArrayLibrary.Array_Contains` (`self.ValidTileTypes`) _type)
              (if (not (`KismetSystemLibrary.IsValid` _unitontile))
                (return true)
                (else
                  (return false)))
              (else
                (return false)))
            (else
              (return false)))
          (else
            (return false)))
        (else
          (return true)))
      (else
        (return false)))
    (else
      (return false))))

(fn `PullCheapestTileOutOfTheDiscoveredList`
  (returns (TilePathData :type "/Game/TurnBasedGame/Blueprints/Grid/Utilities/S_DataPathfinding Structure"))
  (locals (TileIndex :type "IntPoint Structure"))
  (set `local.TileIndex` (`|GetArrayItem` (`self.DiscoveredTileIndexes`)))
  (`KismetArrayLibrary.Array_Remove` (`self.DiscoveredTileSortingCosts`))
  (`KismetArrayLibrary.Array_Remove` (`self.DiscoveredTileIndexes`))
  (`KismetArrayLibrary.Array_Add` (`self.AnalysedTileIndexes`) (`local.TileIndex`))
  (return (`BlueprintMapLibrary.Map_Find` (`self.DataPathfinding`) (`local.TileIndex`))))

(fn `UserConstructionScript`)