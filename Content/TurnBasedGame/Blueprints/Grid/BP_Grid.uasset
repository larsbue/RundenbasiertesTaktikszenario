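; BP_Grid is the tile grid actor for a turn-based game, built in the construction script around the actor's location.
; SpawnGrid sphere-traces each cell for snapped height and BP_GridObstacle tile type, then stores tiles in a map mirrored to a BP_GridVisible child actor.
; Tile states keep a reverse index for lookup, and update calls announce changes.
; It also resolves cursor-to-tile picking and links three pathfinding child actors: general, reachable-tile and AI.
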(fn `AddGridTile`
  (params (Data :type "/Game/TurnBasedGame/Blueprints/Grid/Utilities/S_DataTile Structure"))
  (bind _data_index (break `/Game/TurnBasedGame/Blueprints/Grid/Utilities/S_DataTile` (`local.Data`)))
  (bind _data_index_2 (break `/Game/TurnBasedGame/Blueprints/Grid/Utilities/S_DataTile` (`local.Data`)))
  ;[1 1 1] add the given data to the grid tiles array and update the visuals.
  (`BlueprintMapLibrary.Map_Add` (`self.GridTiles`) _data_index (`local.Data`))
  (`/Game/TurnBasedGame/Blueprints/Grid/Utilities/BP_GridVisible.UpdateTileVisual` (`self.GridVisual`) (`local.Data`))
  (`self.OnTileDataUpdated` _data_index_2))

(fn `AddStateToTile`
  (params (Index :type "IntPoint Structure") (State :type "/Game/TurnBasedGame/Blueprints/Grid/Utilities/E_StateTile Enum" :default "NewEnumerator0"))
  (locals (Data :type "/Game/TurnBasedGame/Blueprints/Grid/Utilities/S_DataTile Structure"))
  (bind _data_index (break `/Game/TurnBasedGame/Blueprints/Grid/Utilities/S_DataTile` (`local.Data`)))
  (bind (_value _returnvalue) (`BlueprintMapLibrary.Map_Find` (`self.GridTiles`) Index))
  (if _returnvalue
    (bind _output_get (set `local.Data` _value))
    (bind _returnvalue_2 (`KismetArrayLibrary.Array_AddUnique` (`.States_12_E157DEAE415E97B85AD1F69681B85DC8` (break `/Game/TurnBasedGame/Blueprints/Grid/Utilities/S_DataTile` _output_get)) State))
    (if (>= _returnvalue_2 0)
      (`BlueprintMapLibrary.Map_Add` (`self.GridTiles`) _data_index (`local.Data`))
      (bind _indexes (`self.GetAllTilesWithState` (`local.State`)))
      (`KismetArrayLibrary.Array_Add` _indexes (`local.Index`))
      (`BlueprintMapLibrary.Map_Add` (`self.TileStateToIndexes`) (`local.State`) (make `/Game/TurnBasedGame/Blueprints/Grid/Utilities/S_IntPointArray` _indexes))
      (`/Game/TurnBasedGame/Blueprints/Grid/Utilities/BP_GridVisible.UpdateTileVisual` (`self.GridVisual`) (`local.Data`))
      (`self.OnTileStateUpdated` (`local.Index`)))))

(fn `CalculateCenterAndBottomLeft`
  (returns (Center :type "Vector Structure") (BottomLeft :type "Vector Structure"))
  (locals (CenterTemp :type "Vector Structure" :default (0.0 0.0 0.0)))
  (bind (_gridtilecount_x _gridtilecount_y) (break `IntPoint` (`self.GridTileCount`)))
  (set `local.CenterTemp` (`/Game/TurnBasedGame/Blueprints/Utilities/BFL_UtilityFunctions.SnapVectorToVector` (`self.GridCenterVector`) (`self.GridTileSize`)))
  (return (`local.CenterTemp`) (- (`local.CenterTemp`) (* (/ (- (`self.GridTileCount`) (`KismetMathLibrary.MakeVector2D` (`KismetMathLibrary.SelectFloat` 0.0 1.0 (`/Game/TurnBasedGame/Blueprints/Utilities/BFL_UtilityFunctions.isIntEven` _gridtilecount_x)) (`KismetMathLibrary.SelectFloat` 0.0 1.0 (`/Game/TurnBasedGame/Blueprints/Utilities/BFL_UtilityFunctions.isIntEven` _gridtilecount_y)))) 2.0) (`self.GridTileSize`)))))

(fn `ClearStateFromTiles`
  (params (State :type "/Game/TurnBasedGame/Blueprints/Grid/Utilities/E_StateTile Enum" :default "NewEnumerator0"))
  (bind _indexes (`self.GetAllTilesWithState` State))
  (for _array_element _indexes
    (`self.RemoveStateFromTile` _array_element State)))

(fn `DestroyGrid`
  (`BlueprintMapLibrary.Map_Clear` (`self.GridTiles`))
  (`/Game/TurnBasedGame/Blueprints/Grid/Utilities/BP_GridVisible.DestroyGridMeshVis` (`self.GridVisual`))
  (`self.OnGridDestroy`))

(fn `GetAllTilesWithState`
  (params (State :type "/Game/TurnBasedGame/Blueprints/Grid/Utilities/E_StateTile Enum" :default "NewEnumerator0"))
  (returns (Indexes :type "Array of IntPoint Structure"))
  (locals (Ret :type "Array of IntPoint Structure"))
  (return (break `/Game/TurnBasedGame/Blueprints/Grid/Utilities/S_IntPointArray` (`BlueprintMapLibrary.Map_Find` (`self.TileStateToIndexes`) State))))

(fn `GetCursorLocationOnGrid`
  (params (PlayerIndex :type Integer))
  (returns (Location :type "Vector Structure"))
  (bind _returnvalue (`GameplayStatics.GetPlayerController` PlayerIndex))
  (bind (_hitresult _returnvalue_2) (`PlayerController.GetHitResultUnderCursorByChannel` _returnvalue "TraceTypeQuery3" false))
  (bind (_worldlocation _worlddirection) (`PlayerController.DeprojectMousePositionToWorld` _returnvalue))
  (bind (_hitresult_2 _returnvalue_3) (`PlayerController.GetHitResultUnderCursorByChannel` _returnvalue "TraceTypeQuery4" true))
  (bind (_t _intersection _returnvalue_4) (`KismetMathLibrary.LinePlaneIntersection` _worldlocation (+ _worldlocation (* _worlddirection 99999999999.0)) (`KismetMathLibrary.MakePlaneFromPointAndNormal` (`self.GridCenterVector`) (0.0 0.0 1.0))))
  (if _returnvalue_3
    (return (`.Location` (`GameplayStatics.BreakHitResult` _hitresult_2)))
    (elif _returnvalue_2
      (return (`.Location` (`GameplayStatics.BreakHitResult` _hitresult)))
      (elif _returnvalue_4
        (return _intersection)
        (else
          (return (-999.0 -999.0 -999.0)))))))

(fn `GetGridShapeData`
  (returns (ReturnValue :type "/Game/TurnBasedGame/Blueprints/Grid/GridRessources/S_DataGridShape Structure"))
  (return (`/Game/TurnBasedGame/Blueprints/Grid/GridRessources/BFL_GridShape.GetShapeData` (`self.GridShape`))))

(fn `GetTileIndexFromLocation`
  (params (Location :type "Vector Structure"))
  (returns (Index :type "IntPoint Structure"))
  (locals (LocationOnGrid :type "Vector Structure") (SnappedLocationOnGrid :type "Vector2D Structure") (TempIndex :type "Vector2D Structure"))
  (set `local.LocationOnGrid` (- Location (`self.GridBottomLeftCornerVector`)))
  (set `local.SnappedLocationOnGrid` (`KismetMathLibrary.Conv_VectorToVector2D` (`/Game/TurnBasedGame/Blueprints/Utilities/BFL_UtilityFunctions.SnapVectorToVector` (`local.LocationOnGrid`) (`self.GridTileSize`))))
  (return (`KismetMathLibrary.Conv_Vector2DToIntPoint` (`KismetMathLibrary.Conv_VectorToVector2D` (/ (`local.SnappedLocationOnGrid`) (`self.GridTileSize`))))))

(fn `GetTileIndexUnderCursor`
  (params (PlayerIndex :type Integer))
  (returns (Index :type "IntPoint Structure"))
  (bind _location (`self.GetCursorLocationOnGrid` PlayerIndex))
  (bind _index (`self.GetTileIndexFromLocation` _location))
  (return _index))

(fn `GetTileLocationFromGridIndex`
  (params (GridIndex :type "IntPoint Structure"))
  (returns (TileLocation :type "Vector Structure"))
  (return (+ (`self.GridBottomLeftCornerVector`) (* (`self.GridTileSize`) (* GridIndex (select `/Game/TurnBasedGame/Blueprints/Grid/GridRessources/E_GridShape` (`self.GridShape`) :`NewEnumerator1` (1.0 1.0) :!type "Vector2D Structure"))))))

(fn `GetTileRotationFromGridIndex`
  (params (GridIndex :type "IntPoint Structure"))
  (returns (TileRotation :type "Rotator Structure"))
  (return))

(fn `GetTileScale`
  (returns (TileScale :type "Vector Structure"))
  (return (/ (`self.GridTileSize`) (`.MeshSize_2_84D275B54683EFCAEB7BF38CDFF98A95` (break `/Game/TurnBasedGame/Blueprints/Grid/GridRessources/S_DataGridShape` (`self.GetGridShapeData`))))))

(fn `IsIndexValid`
  (params (Index :type "IntPoint Structure"))
  (returns (IsValid :type Boolean))
  (if (`BlueprintMapLibrary.Map_Contains` (`self.GridTiles`) Index)
    (return true)))

(fn `IsTileWalkable`
  (params (Index :type "IntPoint Structure"))
  (returns (IsWalkable :type Boolean))
  (return (`/Game/TurnBasedGame/Blueprints/Grid/Utilities/BFL_TileData.IsTileTypeWalkable` (`.Type_6_5F1D582544258A461E8CED80E64FB436` (break `/Game/TurnBasedGame/Blueprints/Grid/Utilities/S_DataTile` (`BlueprintMapLibrary.Map_Find` (`self.GridTiles`) Index))))))

(fn `RemoveGridTile`
  (params (Index :type "IntPoint Structure"))
  (bind _returnvalue (`BlueprintMapLibrary.Map_Remove` (`self.GridTiles`) Index))
  (if _returnvalue
    (`/Game/TurnBasedGame/Blueprints/Grid/Utilities/BP_GridVisible.UpdateTileVisual` (`self.GridVisual`) (make `/Game/TurnBasedGame/Blueprints/Grid/Utilities/S_DataTile` (`local.Index`)))
    (`self.OnTileDataUpdated` (`local.Index`))))

(fn `RemoveStateFromTile`
  (params (Index :type "IntPoint Structure") (State :type "/Game/TurnBasedGame/Blueprints/Grid/Utilities/E_StateTile Enum" :default "NewEnumerator0"))
  (locals (Data :type "/Game/TurnBasedGame/Blueprints/Grid/Utilities/S_DataTile Structure"))
  (bind _data_index (break `/Game/TurnBasedGame/Blueprints/Grid/Utilities/S_DataTile` (`local.Data`)))
  (bind (_value _returnvalue) (`BlueprintMapLibrary.Map_Find` (`self.GridTiles`) Index))
  (if _returnvalue
    (bind _output_get (set `local.Data` _value))
    (bind _returnvalue_2 (`KismetArrayLibrary.Array_RemoveItem` (`.States_12_E157DEAE415E97B85AD1F69681B85DC8` (break `/Game/TurnBasedGame/Blueprints/Grid/Utilities/S_DataTile` _output_get)) State))
    (if _returnvalue_2
      (`BlueprintMapLibrary.Map_Add` (`self.GridTiles`) _data_index (`local.Data`))
      (bind _indexes (`self.GetAllTilesWithState` (`local.State`)))
      (`KismetArrayLibrary.Array_RemoveItem` _indexes (`local.Index`))
      (`BlueprintMapLibrary.Map_Add` (`self.TileStateToIndexes`) (`local.State`) (make `/Game/TurnBasedGame/Blueprints/Grid/Utilities/S_IntPointArray` _indexes))
      (`/Game/TurnBasedGame/Blueprints/Grid/Utilities/BP_GridVisible.UpdateTileVisual` (`self.GridVisual`) (`local.Data`))
      (`self.OnTileStateUpdated` (`local.Index`)))))

(fn `SpawnGrid`
  (params (CenterLocation :type "Vector Structure") (TileSize :type "Vector Structure") (TileCount :type "IntPoint Structure") (Shape :type "/Game/TurnBasedGame/Blueprints/Grid/GridRessources/E_GridShape Enum" :default "NewEnumerator0") (UseEnvironment :type Boolean))
  (locals (X :type Integer) (Y :type Integer) (TileTransform :type "Transform Structure") (Index :type "IntPoint Structure"))
  (bind (_gridtilecount_x _gridtilecount_y) (break `IntPoint` (`self.GridTileCount`)))
  (bind (_tiletransform_location _tiletransform_rotation _tiletransform_scale) (`KismetMathLibrary.BreakTransform` (`local.TileTransform`)))
  (bind _gridtilecount_x_2 (break `IntPoint` (`self.GridTileCount`)))
  (set `self.GridCenterVector` CenterLocation)
  (set `self.GridTileSize` TileSize)
  (set `self.GridTileCount` TileCount)
  (set `self.GridShape` Shape)
  (`|ExecutionSequence`
    (:`then_0`
      (`self.DestroyGrid`)
      (`/Game/TurnBasedGame/Blueprints/Grid/Utilities/BP_GridVisible.InitializeGridMeshVis` (`self.GridVisual`) self)
      (bind (_center _bottomleft) (`self.CalculateCenterAndBottomLeft`))
      (set `self.GridCenterVector` _center)
      (set `self.GridBottomLeftCornerVector` _bottomleft)
      (for _index (range _gridtilecount_x_2)
        (set `local.X` _index)
        (for _index_2 (range _gridtilecount_y)
          (set `local.Y` _index_2)
          (set `local.Index` (make `IntPoint` (`local.X`) (`local.Y`)))
          (set `local.TileTransform` (`KismetMathLibrary.MakeTransform` (`self.GetTileLocationFromGridIndex` (`local.Index`)) (struct) (`self.GetTileScale`)))
          (if (`local.UseEnvironment`)
            (bind (_outlocation _tiletype) (`self.TraceForGround` _tiletransform_location))
            (`self.AddGridTile` (make `/Game/TurnBasedGame/Blueprints/Grid/Utilities/S_DataTile` (`local.Index`) _tiletype (`KismetMathLibrary.MakeTransform` _outlocation (struct) _tiletransform_scale)))
            (else
              (`self.AddGridTile` (make `/Game/TurnBasedGame/Blueprints/Grid/Utilities/S_DataTile` (`local.Index`) "NewEnumerator1" (`local.TileTransform`))))))))
    (:`then_1`
      (`self.OnGridGenerated`))))

(fn `TraceForGround`
  (params (Location :type "Vector Structure"))
  (returns (OutLocation :type "Vector Structure") (TileType :type "/Game/TurnBasedGame/Blueprints/Grid/Utilities/E_TypeTile Enum"))
  (locals (Radius :type "Float (double-precision)") (RetType :type "/Game/TurnBasedGame/Blueprints/Grid/Utilities/E_TypeTile Enum" :default "NewEnumerator0") (RetZ :type "Float (double-precision)" :default 0.0))
  (bind (_location_x _location_y) (`KismetMathLibrary.BreakVector` (`local.Location`)))
  (bind _gridtilesize_x (`KismetMathLibrary.BreakVector` (`self.GridTileSize`)))
  (bind _location (`local.Location`))
  (bind (_gridtilesize_x_2 _gridtilesize_y _gridtilesize_z) (`KismetMathLibrary.BreakVector` (`self.GridTileSize`)))
  (set `local.Radius` (/ _gridtilesize_x 3.0))
  (bind _outhits (`KismetSystemLibrary.SphereTraceMulti` (+ _location (0.0 0.0 1000.0)) (- _location (0.0 0.0 1000.0)) (`local.Radius`) "TraceTypeQuery3" true))
  (if (> (`KismetArrayLibrary.Array_Length` _outhits) 0)
    (set `self.IsHeightFound` false)
    (set `local.RetType` "NewEnumerator1")
    (for _array_element _outhits
      (bind (_bblockinghit _binitialoverlap _time _distance _location_2 _impactpoint _normal _impactnormal _physmat _hitactor) (`GameplayStatics.BreakHitResult` _array_element))
      (bind _asbp_grid_obstacle (cast `/Game/TurnBasedGame/Blueprints/Grid/Utilities/BP_GridObstacle` _hitactor)
        (:`then`
          (set `local.RetType` (`/Game/TurnBasedGame/Blueprints/Grid/Utilities/BP_GridObstacle.Type` _asbp_grid_obstacle))
          (if (`/Game/TurnBasedGame/Blueprints/Grid/Utilities/BP_GridObstacle.UseForTileHeight` _asbp_grid_obstacle)
            (set `self.IsHeightFound` true)
            (bind _returnvalue (`KismetMathLibrary.GridSnap_Float` (- (`.Z` (`KismetMathLibrary.BreakVector3f` _location_2)) (`local.Radius`)) _gridtilesize_z))
            (set `local.RetZ` _returnvalue)))
        (:`CastFailed`
          (if (not (`self.IsHeightFound`))
            (set `local.RetZ` _returnvalue)))))
    (return (`KismetMathLibrary.MakeVector` _location_x _location_y (`local.RetZ`)) (`local.RetType`))
    (else
      (return (`local.Location`) "NewEnumerator0"))))

(fn `UserConstructionScript`
  (set `self.GridVisual` (cast `/Game/TurnBasedGame/Blueprints/Grid/Utilities/BP_GridVisible` (`ChildActorComponent.ChildActor` (`self.ChildActor_GridVisible`)) :!pure true))
  (bind _output_get (set `self.GridPathfinding` (cast `/Game/TurnBasedGame/Blueprints/Grid/BP_GridPathfinding` (`ChildActorComponent.ChildActor` (`self.ChildActor_Pathfinding`)) :!pure true)))
  (set `/Game/TurnBasedGame/Blueprints/Grid/BP_GridPathfinding.Grid` self _output_get)
  (bind _output_get_2 (set `self.GridPathfinding_ReachableTile` (cast `/Game/TurnBasedGame/Blueprints/Grid/BP_GridPathfinding` (`ChildActorComponent.ChildActor` (`self.ChildActor_Pathfinding_Reachables`)) :!pure true)))
  (set `/Game/TurnBasedGame/Blueprints/Grid/BP_GridPathfinding.Grid` self _output_get_2)
  (bind _output_get_3 (set `self.GridPathfinding_AI` (cast `/Game/TurnBasedGame/Blueprints/Grid/BP_GridPathfinding` (`ChildActorComponent.ChildActor` (`self.ChildActor_Pathfinding_AI`)) :!pure true)))
  (set `/Game/TurnBasedGame/Blueprints/Grid/BP_GridPathfinding.Grid` self _output_get_3)
  (`self.SpawnGrid` (`self.K2_GetActorLocation`) (`self.GridTileSize`) (`self.GridTileCount`) (`self.GridShape`) true))