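; BP_GridObstacle is an editor-visible, in-game hidden marker that affects grid generation in the turn-based game.
; Its construction script takes mesh and flat material from the selected Shape's data and tints them by tile Type, such as obstacle, movement cost or flying-only.
; It sets overlap and block responses on two custom trace channels, intended to affect line of sight and grid passability.
; All event graph events are empty.
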(fn `UserConstructionScript`
  (bind _staticmesh (`self.StaticMesh`))
  (bind _staticmesh_2 (`self.StaticMesh`))
  (bind (_data_meshsize _data_mesh _data_meshmaterial _data_flatmesh _data_flatmaterial) (break `/Game/TurnBasedGame/Blueprints/Grid/GridRessources/S_DataGridShape` (`/Game/TurnBasedGame/Blueprints/Grid/GridRessources/BFL_GridShape.GetShapeData` (`self.Shape`))))
  ;[1 1 1] sets the mesh and material of the obstacle as described in the shape structure.
  (`StaticMeshComponent.SetStaticMesh` _staticmesh _data_mesh)
  (`PrimitiveComponent.SetMaterial` _staticmesh 0 _data_flatmaterial)
  ;[1 1 1] colors the obstacle according to its type
  (`MeshComponent.SetVectorParameterValueOnMaterials` _staticmesh "Color" (`KismetMathLibrary.Conv_LinearColorToVector` (select `/Game/TurnBasedGame/Blueprints/Grid/Utilities/E_TypeTile` (`self.Type`) :`NewEnumerator1` (struct :`R` 1.0 :`G` 1.0 :`B` 1.0 :`A` 1.0) :`NewEnumerator2` (struct :`R` 1.0 :`A` 1.0) :`NewEnumerator3` (struct :`R` 0.958333 :`G` 0.545784 :`B` 0.154731 :`A` 1.0) :`NewEnumerator4` (struct :`R` 0.385417 :`G` 0.16473 :`B` 0.042155 :`A` 1.0) :`NewEnumerator5` (struct :`R` 0.723958 :`G` 0.303675 :`A` 1.0) :!type "LinearColor Structure")))
  (`MeshComponent.SetScalarParameterValueOnMaterials` _staticmesh "IsFilled" 1.0)
  ;[1 1 1] block line of sight AND grid generation to make it non passable. also hide it ingame because its ugly otherwise.
  (`PrimitiveComponent.SetCollisionResponseToChannel` _staticmesh_2 "ECC_GameTraceChannel1" "ECR_Overlap")
  (`PrimitiveComponent.SetCollisionResponseToChannel` _staticmesh_2 "ECC_GameTraceChannel4" "ECR_Block")
  (`self.SetActorHiddenInGame` true))